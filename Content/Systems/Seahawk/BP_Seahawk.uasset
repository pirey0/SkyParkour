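; BP_Seahawk is a player-flown aircraft that moves by physics forces and fires shells from a child fireworks launcher on left click.
; Move axes and held jump apply mass-independent forces to Box, while the look axis drives yaw.
; Tick spins the top and tail arrows faster with vertical speed.
; It also tilts WholeBody from local forward and sideways velocity, separating visual banking from the actor's rotation.
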(event `self.ReceiveTick`
  (params (DeltaSeconds :type "Float (single-precision)"))
  (bind _returnvalue (`self.GetVelocity`))
  ;[1 1 1] Tick
  (`|ExecutionSequence`
    (:`then_0`
      (if (`self.jumpHeld`)
        (`PrimitiveComponent.AddForce` (`self.Box`) (* (`self.GetActorUpVector`) (`self.MoveForce`)) "None" true)))
    (:`then_1`
      (`SceneComponent.K2_AddLocalRotation` (`self.ArrowTop`) (* (`KismetMathLibrary.MakeRotator` (+ (`KismetMathLibrary.Abs` (.z (`self.GetVelocity`))) 400.0)) DeltaSeconds) false false)
      (`SceneComponent.K2_AddLocalRotation` (`self.ArrowTail`) (* (`KismetMathLibrary.MakeRotator` (+ (`KismetMathLibrary.Abs` (.z (`self.GetVelocity`))) 400.0)) DeltaSeconds) false false))
    (:`then_2`
      (`self.K2_AddActorLocalRotation` (* (`KismetMathLibrary.MakeRotator` 0.0 0.0 (* (`self.TurnSpeed`) (`self.YawRotValue`))) DeltaSeconds)))
    (:`then_3`
      (`SceneComponent.K2_SetRelativeRotation` (`self.WholeBody`) (`KismetMathLibrary.MakeRotator` (`KismetMathLibrary.MapRangeClamped` (* (`KismetMathLibrary.Dot_VectorVector` _returnvalue (`self.GetActorRightVector`)) (`self.RollRotValue`)) -300.0 300.0 -50.0 50.0) (`KismetMathLibrary.MapRangeClamped` (* (`KismetMathLibrary.Dot_VectorVector` _returnvalue (`self.GetActorForwardVector`)) (`self.PitchRotValue`)) 300.0 -300.0 -50.0 50.0)) false true))))

(event `InputAxis|MoveForward/Backwards`
  (params (AxisValue :type "Float (single-precision)"))
  (`PrimitiveComponent.AddForce` (`self.Box`) (* (`self.GetActorForwardVector`) (* AxisValue (`self.MoveForce`))) "None" true))

(event `InputAxis|MoveRight/Left`
  (params (AxisValue :type "Float (single-precision)"))
  (`PrimitiveComponent.AddForce` (`self.Box`) (* (`self.GetActorRightVector`) (* AxisValue (`self.MoveForce`))) "None" true))

(event `InputAction|JumpAction`
  (params (Key :type "Key Structure"))
  (:`Pressed`
    (set `self.jumpHeld` true))
  (:`Released`
    (set `self.jumpHeld` false)))

(event `InputAxis|LookLeft/Right`
  (params (AxisValue :type "Float (single-precision)"))
  (set `self.YawRotValue` AxisValue))

(event `Key|LeftMouseButton`
  (params (Key :type "Key Structure"))
  (:`Pressed`
    (bind _asts_fireworks_launcher (cast `/Game/Systems/TS_Fireworks/Blueprints/TS_FireworksLauncher` (`ChildActorComponent.ChildActor` (`self.ChildFireworkLaucher`))))
    (`/Game/Systems/TS_Fireworks/Blueprints/TS_FireworksLauncher.LaunchShell` _asts_fireworks_launcher)))

(fn `UserConstructionScript`)