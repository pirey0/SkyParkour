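; Cutscene helper Blueprint that shows a widget on screen and fades it in and out.
; Spawn creates a widget of the configured class, adds it to the viewport and starts it fully transparent.
; FadeIn and FadeOut play one timeline forward or in reverse at a given play rate to drive the widget's render opacity.
; Terminate removes the widget from its parent.
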(event `Spawn`
  (bind _returnvalue (`|CreateWidget` (`self.WidgetClass`)))
  (set `self.Wdiget` _returnvalue)
  (`UserWidget.AddToViewport` _returnvalue 0)
  (`Widget.SetRenderOpacity` (`self.Wdiget`) 0.0))

(event `FadeIn`
  (params (`Play Rate` :type "Float (double-precision)"))
  (`TimelineComponent.SetPlayRate` (`self.FadeTimeLine`) `Play Rate`)
  (bind (_direction _linear) (`Timeline|FadeTimeLine` :!via `PlayFromStart` :!label _label)
    (:`Update`
      (`Widget.SetRenderOpacity` (`self.Wdiget`) _linear))))

(event `FadeOut`
  (params (PlayRate :type "Float (double-precision)"))
  (`TimelineComponent.SetPlayRate` (`self.FadeTimeLine`) PlayRate)
  (goto _label :!via `ReverseFromEnd`))

(event `Terminate`
  (`Widget.RemoveFromParent` (`self.Wdiget`)))

(fn `UserConstructionScript`)