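; Night controller that limits how long the player survives outside a safespot at night.
; While the Clock reports night, Tick refills the survival timer inside a safespot and counts it down by delta time otherwise.
; When time runs out, the player pawn teleports to the Respawn location and is flagged as in a safespot.
; A hard-coded true branch leaves the alternative level-reload death unreachable.
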(event `self.ReceiveBeginPlay`
  (set `self.SurvivalTimeLeft` (`self.maxSurvivalTime`)))

(event `self.ReceiveTick`
  (params (DeltaSeconds :type "Float (single-precision)"))
  (if (`/Game/Blueprints/ArtPrototype/BP_SkySystem.NightTime` (`self.Clock`))
    (if (`self.PlayerInSafespot`)
      ;[1 1 1] Reset Survival Time in Safespot
      (set `self.SurvivalTimeLeft` (`self.maxSurvivalTime`))
      (elif (> (`self.SurvivalTimeLeft`) 0.0)
        ;[1 1 1] Reduce Survival Time by time passed since last tick
        (set `self.SurvivalTimeLeft` (- (`self.SurvivalTimeLeft`) (`GameplayStatics.GetWorldDeltaSeconds`)))
        (elif true
          (`Actor.K2_TeleportTo` :`self` (`GameplayStatics.GetPlayerPawn` 0) :`DestLocation` (`Actor.K2_GetActorLocation` (`self.Respawn`)))
          (set `self.PlayerInSafespot` true)
          (`KismetSystemLibrary.PrintString` "player deaded")
          (else
            ;[1 1 1] Reload Scene (Player dies)
            (bind _returnvalue (`GameplayStatics.GetCurrentLevelName` true))
            (`GameplayStatics.OpenLevel` (`KismetStringLibrary.Conv_StringToName` _returnvalue))
            (`KismetSystemLibrary.PrintString` "Died in darkness")))))))