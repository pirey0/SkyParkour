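; Prototype weather controller actor that toggles rain on and off with the 7 key.
; ToggleRain switches the rain particle system and looping sound, sets the direction of change and enables Tick.
; Tick steps RainLevel by a fixed per-frame amount into the MP_Global material parameter collection for materials to read.
; Tick disables itself once the level passes 0 or 1, without clamping the value.
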(event `self.ReceiveBeginPlay`
  (`self.EnableInput` (`GameplayStatics.GetPlayerController` 0)))

(event `Key|Seven`
  (params (Key :type "Key Structure"))
  (:`Pressed`
    (bind _isa (`/Engine/EditorBlueprintResources/StandardMacros.FlipFlop`)
      (:`A`
        _)
      (:`B`
        _))
    (`self.ToggleRain` _isa)))

(event `self.ReceiveTick`
  (params (DeltaSeconds :type "Float (single-precision)"))
  (bind _rainlevel (`self.RainLevel`))
  (bind _output_get (set `self.RainLevel` (+ (`self.RainLevel`) (`self.ChangeRate`))))
  (`KismetMaterialLibrary.SetScalarParameterValue` "/Game/Environment/03_Materials/MaterialParamCollections/MP_Global.MP_Global" "RainLevel" _output_get)
  (if (or (> _rainlevel 1.0) (< _rainlevel 0.0))
    (`self.SetActorTickEnabled` false)))

(event `ToggleRain`
  (params (enable :type Boolean))
  (if enable
    (`ActorComponent.SetActive` (`self.Rain_PS`) true false)
    (`AudioComponent.Play` (`self.Rain_loop`) 0.0)
    (set `self.ChangeRate` 0.1)
    (`self.SetActorTickEnabled` true)
    (else
      (`ActorComponent.SetActive` (`self.Rain_PS`) false false)
      (`AudioComponent.Stop` (`self.Rain_loop`))
      (set `self.ChangeRate` -0.1)
      (`self.SetActorTickEnabled` true))))

(fn `UserConstructionScript`)