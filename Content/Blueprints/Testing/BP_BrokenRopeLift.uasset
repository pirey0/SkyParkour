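; BP_BrokenRopeLift is a testing interactable for a broken rope lift that is repaired when the interactor carries the required items.
; A required-inventory component fills from RequiredElements shortly after BeginPlay.
; On Interact, it fetches the interactor's inventory through BPI_Container and checks it contains every requirement.
; Repair spawns a BP_Screwdriver at the lift's root transform and destroys the lift; failures only print debug strings.
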(event `self.ReceiveBeginPlay`
  (`KismetSystemLibrary.Delay` 0.2)
  (`/Game/Blueprints/Inventory/BP_InventoryComp.PopulateFromDTUtilArray` (`self.BP_RequiredInventoryComp`) (`self.RequiredElements`)))

(event `/Game/Blueprints/Interface/BPI_Interact.Interact`
  (params (Actor :type "Actor Object Reference"))
  ;[1 1 1] Interact
  (if (`self.repaired`)
    _
    (elif (`KismetSystemLibrary.DoesImplementInterface` Actor "/Game/Blueprints/Interface/BPI_Container.BPI_Container_C")
      (bind _inventorycomp (message `/Game/Blueprints/Interface/BPI_Container.GetInventoryComponent` Actor))
      (bind _doescontain (`/Game/Blueprints/Inventory/BP_InventoryComp.ContainsAllInInventory` _inventorycomp (`self.BP_RequiredInventoryComp`)))
      (if _doescontain
        (`self.RepairRopeLift`)
        (else
          (`KismetSystemLibrary.PrintString` "You do not have the correct Object to open")))
      (else
        (`KismetSystemLibrary.PrintString` "Interactor does not implement Container")))))

(event `RepairRopeLift`
  (if (`self.repaired`)
    (`KismetSystemLibrary.PrintString` "Already repaired")
    (else
      (set `self.repaired` true)
      (`|SpawnActorFromClass` "/Game/Blueprints/Testing/BP_Screwdriver.BP_Screwdriver_C" (`SceneComponent.K2_GetComponentToWorld` (`self.DefaultSceneRoot`)) "AlwaysSpawn" "OverrideRootScale" null (struct) null)
      (`self.K2_DestroyActor`))))

(event `/Game/Blueprints/Interface/BPI_Interact.EndInteract`
  (params (Actor :type "Actor Object Reference")))

(fn `UserConstructionScript`)