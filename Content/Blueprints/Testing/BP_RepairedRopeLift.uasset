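; Test Blueprint for a repaired rope lift, built from two cable components and exposing position data for the lift's span.
; The construction script and BeginPlay both attach the cable ends to the End component and StaticMesh3.
; GetStartPosition returns the StartPosition world location, and GetDisplacement returns the world-space vector from Start to End.
; Interact and EndInteract events are empty stubs.
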(event `self.ReceiveBeginPlay`
  (`CableComponent.SetAttachEndToComponent` (`self.Cable`) (`self.End`) "None")
  (`CableComponent.SetAttachEndToComponent` (`self.Cable1`) (`self.StaticMesh3`) "None"))

(event `/Game/Blueprints/Interface/BPI_Interact.Interact`
  (params (Actor :type "Actor Object Reference")))

(event `/Game/Blueprints/Interface/BPI_Interact.EndInteract`
  (params (Actor :type "Actor Object Reference")))

(fn `GetDisplacement`
  (returns (Displacement :type "Vector Structure"))
  (return (- (`SceneComponent.K2_GetComponentLocation` (`self.End`)) (`SceneComponent.K2_GetComponentLocation` (`self.Start`)))))

(fn `GetStartPosition`
  (returns (Position :type "Vector Structure"))
  (return (`SceneComponent.K2_GetComponentLocation` (`self.StartPosition`))))

(fn `UserConstructionScript`
  (`CableComponent.SetAttachEndToComponent` (`self.Cable`) (`self.End`) "None")
  (`CableComponent.SetAttachEndToComponent` (`self.Cable1`) (`self.StaticMesh3`) "None"))