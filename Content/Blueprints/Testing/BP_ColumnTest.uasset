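; BP_ColumnTest is a test actor that builds a segmented column from spline meshes along its Spline component.
; The construction script puts BotMesh on the first segment, repeats Mesh on the middle segments, and caps the last with TopMesh when more than two spline points exist.
; CreateSplineMeshAtIndex adds each spline mesh component, attaches it to Scene and bends it using the local locations and tangents of adjacent points.
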(fn `CreateSplineMeshAtIndex`
  (params (Mesh :type "StaticMesh Object Reference") (Index :type Integer))
  (bind _spline (`self.Spline`))
  (bind (_location _tangent) (`SplineComponent.GetLocationAndTangentAtSplinePoint` _spline (+ Index 1) "Local"))
  (bind (_location_2 _tangent_2) (`SplineComponent.GetLocationAndTangentAtSplinePoint` _spline Index "Local"))
  (bind _returnvalue (`AddComponent|NODE_AddSplineMeshComponent-1` :`bManualAttachment` true))
  (`|ExecutionSequence`
    (:`then_0`
      (`StaticMeshComponent.SetStaticMesh` _returnvalue Mesh))
    (:`then_1`
      (`SceneComponent.K2_AttachToComponent` _returnvalue (`self.Scene`) "None" "KeepRelative" "KeepRelative" "KeepRelative" true))
    (:`then_2`
      (`SplineMeshComponent.SetStartAndEnd` _returnvalue _location_2 _tangent_2 _location _tangent true))))

(fn `UserConstructionScript`
  (bind _returnvalue (`SplineComponent.GetNumberOfSplinePoints` (`self.Spline`)))
  (bind _returnvalue_2 (- _returnvalue 2))
  (`|ExecutionSequence`
    (:`then_0`
      (`self.CreateSplineMeshAtIndex` (`self.BotMesh`)))
    (:`then_1`
      (for _index (range 1 (+ (- _returnvalue 3) 1))
        (`self.CreateSplineMeshAtIndex` (`self.Mesh`) _index)))
    (:`then_2`
      (if (> _returnvalue_2 0)
        (`self.CreateSplineMeshAtIndex` (`self.TopMesh`) _returnvalue_2)))))