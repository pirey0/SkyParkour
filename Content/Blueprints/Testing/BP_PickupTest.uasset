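; BP_PickupTest is a test pickup actor that spins around its yaw axis every tick at RotationSpeed.
; On overlap it checks whether the other actor implements BPI_Container and fetches that actor's inventory component through the interface.
; It looks up its item row from a data table handle, adds one to that inventory and destroys itself on success.
; Debug strings report overlaps, a missing interface or a missing row.
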(event `self.ReceiveActorBeginOverlap`
  (params (OtherActor :type "Actor Object Reference"))
  (bind (_inventoryobject_row_datatable _inventoryobject_row_rowname) (break `DataTableRowHandle` (`self.InventoryObject Row`)))
  (`KismetSystemLibrary.PrintString` (`KismetStringLibrary.Concat_StrStr` "Overlapped with " (`KismetSystemLibrary.GetDisplayName` OtherActor)) true false (struct :`R` 1.0 :`G` 1.0 :`B` 1.0 :`A` 1.0))
  (if (`KismetSystemLibrary.DoesImplementInterface` OtherActor "/Game/Blueprints/Interface/BPI_Container.BPI_Container_C")
    (bind _inventorycomp (message `/Game/Blueprints/Interface/BPI_Container.GetInventoryComponent` OtherActor))
    (bind _returnvalue (`|GetDataTableRow` _inventoryobject_row_datatable _inventoryobject_row_rowname)
      (:`then`
        (bind _wasadded (`/Game/Blueprints/Inventory/BP_InventoryComp.AddToInventory` _inventorycomp (make `/Game/Blueprints/Inventory/S_InventoryGroup` _returnvalue 1) true))
        (if _wasadded
          (`self.K2_DestroyActor`)))
      (:`RowNotFound`
        (`KismetSystemLibrary.PrintString` "Data Table Row not Found" true false (struct :`R` 1.0 :`G` 1.0 :`B` 1.0 :`A` 1.0))))
    (else
      (`KismetSystemLibrary.PrintString` "Target does not implement BPI Container" true false (struct :`R` 1.0 :`G` 1.0 :`B` 1.0 :`A` 1.0)))))

(event `self.ReceiveTick`
  (params (DeltaSeconds :type "Float (single-precision)"))
  (`self.K2_AddActorLocalRotation` (`KismetMathLibrary.MakeRotator` 0.0 0.0 (* DeltaSeconds (`self.RotationSpeed`)))))

(fn `UserConstructionScript`)