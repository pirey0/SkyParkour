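; Base is the player's home area, with a trigger box, a bed child actor and an artifact display.
; On BeginPlay it passes its DestroyBlock reference to the Bed.
; Entering the box plays a home jingle, throttled by a ten-second delay.
; The overlap also asks BP_DesignGameMode for an artifact on reaching base; a valid one reveals the base's artifact and destroys the returned object's owner.
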(event `self.ReceiveBeginPlay`
  ;[1 1 1] play sound max every 10 sec
  (`|ExecutionSequence`
    (:`then_0`
      (bind _asbed (cast `/Game/Blueprints/DesignPrototype/Bed` (`ChildActorComponent.ChildActor` (`self.Bed`))))
      (set `/Game/Blueprints/DesignPrototype/Bed.DestroyBlocks` (`self.DestroyBlock`) _asbed))
    (:`then_1`
      (set `self.playSound` true))))

(event `self.Box.OnComponentBeginOverlap`
  (params (OverlappedComponent :type "PrimitiveComponent Object Reference") (OtherActor :type "Actor Object Reference") (OtherComp :type "PrimitiveComponent Object Reference") (OtherBodyIndex :type Integer) (bFromSweep :type Boolean) (SweepResult :type "HitResult Structure (by ref)"))
  (`|ExecutionSequence`
    (:`then_0`
      ;[1 1 1] play sound max every 10 sec
      (if (`self.playSound`)
        (`GameplayStatics.PlaySound2D` "/Game/Blueprints/DesignPrototype/Sounds/homeJingle.homeJingle" 1.0 1.0 0.0 null null)
        (set `self.playSound` false)
        (`KismetSystemLibrary.Delay` 10.0)
        (set `self.playSound` true)))
    (:`then_1`
      ;[1 1 1] place artifact on first enter
      (bind _asbp_design_game_mode (cast `/Game/Blueprints/DesignPrototype/BP_DesignGameMode` (`GameplayStatics.GetGameMode`)))
      (bind _artifact (`/Game/Blueprints/DesignPrototype/BP_DesignGameMode.GetArtifactOnReachedBase` _asbp_design_game_mode))
      (if (`KismetSystemLibrary.IsValid` _artifact)
        (`SceneComponent.SetVisibility` (`self.Artifact`) true false)
        (`self.K2_DestroyActor` (`ActorComponent.GetOwner` _artifact))))))

(fn `UserConstructionScript`)