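; BP_CloudBase is a prototype base actor for drifting clouds.
; Each tick it offsets its root component along local Y by Speed scaled by delta time, with no sweep.
; A helper function gives a supplied mesh component a random mesh from CloudMeshes and applies MaterialInst to its first material slot.
; Nothing in this Blueprint calls that helper, and the construction script is empty.
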(event `self.ReceiveTick`
  (params (DeltaSeconds :type "Float (single-precision)"))
  (`SceneComponent.K2_AddRelativeLocation` (`self.DefaultSceneRoot`) (* (`KismetMathLibrary.MakeVector` 0.0 (`self.Speed`)) DeltaSeconds) false false))

(fn `GetRandomCloudMesh`
  (returns (Mesh :type "StaticMesh Object Reference"))
  (bind _cloudmeshes (`self.CloudMeshes`))
  (return (`|GetArrayItem` _cloudmeshes (`KismetMathLibrary.RandomInteger` (`KismetArrayLibrary.Array_Length` _cloudmeshes)))))

(fn `GiveMeshComponentRandomCloud`
  (params (Component :type "StaticMeshComponent Object Reference"))
  (`StaticMeshComponent.SetStaticMesh` Component (`self.GetRandomCloudMesh`))
  (`PrimitiveComponent.SetMaterial` Component 0 (`self.MaterialInst`)))

(fn `UserConstructionScript`)