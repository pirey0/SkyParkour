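; Prototype cloud actor that shows a random cloud mesh and drifts steadily.
; On BeginPlay it picks a mesh from CloudMeshes and applies MaterialInst to its first material slot.
; Each Tick moves the mesh component along its relative Y axis by Speed scaled by delta time, without sweeping.
; The graph has no wrap-around or despawn logic, and the construction script is empty.
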(event `self.ReceiveBeginPlay`
  (bind _cloudmeshes (`self.CloudMeshes`))
  (`StaticMeshComponent.SetStaticMesh` (`self.StaticMesh`) (`|GetArrayItem` _cloudmeshes (`KismetMathLibrary.RandomIntegerInRange` 0 (- (`KismetArrayLibrary.Array_Length` _cloudmeshes) 1))))
  (`PrimitiveComponent.SetMaterial` (`self.StaticMesh`) 0 (`self.MaterialInst`))
  (`PrimitiveComponent.SetMaterial` (`self.StaticMesh`) 0 (`self.MaterialInst`)))

(event `self.ReceiveTick`
  (params (DeltaSeconds :type "Float (single-precision)"))
  (`SceneComponent.K2_AddRelativeLocation` (`self.StaticMesh`) (* (`KismetMathLibrary.MakeVector` 0.0 (`self.Speed`)) DeltaSeconds) false false))

(fn `UserConstructionScript`)