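; BP_Boids is a prototype boids actor that periodically picks a new target point.
; From BeginPlay, a looping RetriggerableDelay refreshes MTarget every ten seconds as the actor's current location plus a random vector scaled by MRadius.
; Each random component spans zero to one, so targets fall only on the positive side of each axis.
; The Blueprint graphs contain no movement or flocking logic.
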(event `self.ReceiveBeginPlay`
  (set `self.m_Target` (+ (`self.K2_GetActorLocation`) (* (`KismetMathLibrary.MakeVector` (`KismetMathLibrary.RandomFloat`) (`KismetMathLibrary.RandomFloat`) (`KismetMathLibrary.RandomFloat`)) (`KismetMathLibrary.Conv_IntToDouble` (`self.m_Radius`)))) :!label _label)
  (`KismetSystemLibrary.RetriggerableDelay` 10.0)
  (goto _label))

(fn `UserConstructionScript`)