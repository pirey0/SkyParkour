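; BP_PortalSpawner is a prototype actor that spawns a row of level portals, one for each map name returned by GetAllMapNamesP.
; On BeginPlay it loops over that list and spawns a BP_Portal per entry, always spawning regardless of collision.
; Portals share the spawner's rotation and step along its right vector at fixed spacing, each receiving its map name as SceneToLoad.
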(event `self.ReceiveBeginPlay`
  (bind _returnvalue (`MapNamesBPLibrary.GetAllMapNames_p`))
  (bind _returnvalue_2 (`self.K2_GetActorRotation`))
  (for _index (range (`KismetArrayLibrary.Array_Length` _returnvalue))
    (`|SpawnActorFromClass` "/Game/Blueprints/DesignPrototype/BP_Portal.BP_Portal_C" (`KismetMathLibrary.MakeTransform` (+ (* (`KismetMathLibrary.GetRightVector` _returnvalue_2) (* _index 200.0)) (`self.K2_GetActorLocation`)) _returnvalue_2) "AlwaysSpawn" "OverrideRootScale" null (`KismetStringLibrary.Conv_StringToName` (`|GetArrayItem` _returnvalue _index)) null)))

(fn `UserConstructionScript`)