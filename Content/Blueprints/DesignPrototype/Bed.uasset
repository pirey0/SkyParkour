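; Prototype bed interactable that plays a sleep fade, with a one-time collapse event on first use.
; Interact, guarded by an InUse flag, creates a sleep HUD widget and drives its opacity through fade-in and fade-out timelines.
; Between fades, the first sleep plays a collapse sound, turns on a referenced light and destroys the DestroyBlocks actors.
; The overlay is removed and the bed released afterwards; EnterBed is an empty stub.
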(event `self.ReceiveBeginPlay`
  (set `self.triggerEventOnFirstTimeUsage` true))

(event `/Game/Blueprints/Interface/BPI_Interact.Interact`
  (params (Actor :type "Actor Object Reference"))
  ;[1 1 1] bool check if bed is already in use
  (if (not (`self.inUse`))
    (set `self.inUse` true)
    ;[1 1 1] Regular Going to Sleep
    (bind _returnvalue (`|CreateWidget` "/Game/UI/WBP_SleepFade_HUD.WBP_SleepFade_HUD_C"))
    (bind _output_get (set `self.ScreenOverlay` _returnvalue))
    (`UserWidget.AddToViewport` _output_get 0)
    (bind (_direction _opacity) (`Timeline|SleepingIN` :!via `PlayFromStart`)
      (:`Update`
        (`Widget.SetRenderOpacity` (`self.ScreenOverlay`) _opacity))
      (:`Finished`
        ;[1 1 1] Trigger Event or not?
        (if (`self.triggerEventOnFirstTimeUsage`)
          ;[1 1 1] Destruction on Sleep Event
          (`GameplayStatics.PlaySound2D` "/Game/StarterContent/Audio/Collapse02.Collapse02" 1.0 1.0 0.0 null null)
          (`/Game/Blueprints/DesignPrototype/BP_DayNighTimeTrigger.TurnOn` (`self.TurnOnLight`))
          (for _array_element (`self.DestroyBlocks`)
            (`self.K2_DestroyActor` _array_element))
          (set `self.triggerEventOnFirstTimeUsage` false))
        ;[1 1 1] Regular Waking Up
        (`KismetSystemLibrary.Delay` 1.0)
        (bind (_direction_2 _opacity_2) (`Timeline|SleepingOUT` :!via `PlayFromStart`)
          (:`Update`
            (`Widget.SetRenderOpacity` (`self.ScreenOverlay`) _opacity_2))
          (:`Finished`
            (`Widget.RemoveFromParent` (`self.ScreenOverlay`))
            (set `self.inUse` false)))))))

(fn `EnterBed`)

(fn `UserConstructionScript`)