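; Main menu game mode that shows the mouse cursor and puts the WBP_MainMenu widget on screen at BeginPlay.
; It also carries exploration state: interactable structures register toward a total, finds raise an activated count, and a getter formats both as progress text.
; A found artifact is stored with a flag, and a base-reached call sets its own flag and returns that artifact if found.
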(event `self.ReceiveBeginPlay`
  (set `PlayerController.bShowMouseCursor` true (`GameplayStatics.GetPlayerController` 0))
  (bind _returnvalue (`|CreateWidget` "/Game/UI/WBP_MainMenu.WBP_MainMenu_C"))
  (`UserWidget.AddToViewport` _returnvalue 0))

(fn `FindArtifact`
  (params (Artifact :type "StaticMeshComponent Object Reference"))
  (set `self.Artifact` Artifact)
  (set `self.foundArtifact` true))

(fn `FindInteractableStructure`
  (set `self.numberOfStructuresActivated` (+ (`self.numberOfStructuresActivated`) 1)))

(fn `GetArtifactOnReachedBase`
  (returns (Artifact :type "StaticMeshComponent Object Reference"))
  (set `self.reachedBase` true)
  (if (`self.foundArtifact`)
    (return (`self.Artifact`))))

(fn `GetInteractableStructureOnFindText`
  (returns (DisplayText :type Text))
  (return (`KismetTextLibrary.Conv_StringToText` (`KismetStringLibrary.Concat_StrStr` (`KismetStringLibrary.Concat_StrStr` (`KismetStringLibrary.Concat_StrStr` (`KismetStringLibrary.Concat_StrStr` "( " (`KismetStringLibrary.Conv_IntToString` (`self.numberOfStructuresActivated`))) " / ") (`KismetStringLibrary.Conv_IntToString` (`self.numberOfStructuresMax`))) " )"))))

(fn `RegisterInteractableStructure`
  (set `self.numberOfStructuresMax` (+ (`self.numberOfStructuresMax`) 1)))

(fn `UserConstructionScript`)