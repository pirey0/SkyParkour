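; Day/night trigger prototype that rotates a light source to change the time of day.
; Trigger overlap or ChangeDaytime plays a timeline from the start, only while IsDay is true.
; The timeline drives the light's pitch and refreshes the sky sphere material each update, then flips IsDay on finish.
; A separate TurnOn event plays the same timeline in reverse from the end, without checking IsDay.
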(event `ChangeDaytime`
  (if (`self.IsDay`) :!label _label
    (bind (_direction _floatoutput) (`Timeline|Timeline_0` :!via `PlayFromStart` :!label _label_2)
      (:`Update`
        (`self.K2_SetActorRotation` (`self.LightSource`) (`KismetMathLibrary.MakeRotator` 0.0 _floatoutput) false)
        (`/Engine/EngineSky/BP_Sky_Sphere.RefreshMaterial` (`self.SkySphere`)))
      (:`Finished`
        (set `self.IsDay` (not (`self.IsDay`)))))))

(event `self.Trigger.OnComponentBeginOverlap`
  (params (OverlappedComponent :type "PrimitiveComponent Object Reference") (OtherActor :type "Actor Object Reference") (OtherComp :type "PrimitiveComponent Object Reference") (OtherBodyIndex :type Integer) (bFromSweep :type Boolean) (SweepResult :type "HitResult Structure (by ref)"))
  (goto _label))

(event `TurnOn`
  (goto _label_2 :!via `ReverseFromEnd`))

(fn `UserConstructionScript`)