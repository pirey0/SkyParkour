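; Cloud handler actor that keeps a set number of randomly varied cloud actors within a box volume.
; On BeginPlay it scatters clouds through the Box with random class, yaw and scale, passing each a shared speed and material.
; Each Tick, a bounds macro finds the first cloud outside the actor's bounds, destroys it and spawns a replacement in a thin slice near the box's negative-Y edge.
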(event `self.ReceiveBeginPlay`
  ;[1 1 1] Begin Play Spawn Clouds
  (`KismetArrayLibrary.Array_Clear` (`self.Clouds`))
  (for _ (range 1 (+ (`self.Amount`) 1))
    (bind _actor (`self.CreateCloud` false))
    (`KismetArrayLibrary.Array_Add` (`self.Clouds`) _actor)))

(event `self.ReceiveTick`
  (params (DeltaSeconds :type "Float (single-precision)"))
  (bind (_origin _boxextent) (`self.GetActorBounds` false))
  (bind _clouds (`self.Clouds`))
  (for (_array_element _array_index) _clouds
    (`self.IsInsideBounds` _origin _boxextent (`self.K2_GetActorLocation` _array_element)
      (:`False`
        (`self.K2_DestroyActor` _array_element)
        (`KismetArrayLibrary.Array_Remove` _clouds _array_index)
        (bind _actor (`self.CreateCloud` true))
        (`KismetArrayLibrary.Array_Add` (`self.Clouds`) _actor)
        (break)))))

(fn `CreateCloud`
  (params (ForceToRight :type Boolean))
  (returns (Actor :type "Actor Object Reference"))
  (bind _cloudssources (`self.CloudsSources`))
  (bind (_scalesize_x _scalesize_y) (`KismetMathLibrary.BreakVector2D` (`self.ScaleSize`)))
  (bind (_origin _boxextent) (`KismetSystemLibrary.GetComponentBounds` (`self.Box`)))
  (bind _returnvalue (`|SpawnActorFromClass` (`|GetArrayItem` _cloudssources (`KismetMathLibrary.RandomInteger` (`KismetArrayLibrary.Array_Length` _cloudssources))) (`KismetMathLibrary.MakeTransform` (select `bool` ForceToRight :`false` (`KismetMathLibrary.RandomPointInBoundingBox` _origin _boxextent) :`true` (`KismetMathLibrary.RandomPointInBoundingBox` (- _origin (`KismetMathLibrary.MakeVector` 0.0 (* (.y _boxextent) 0.95))) (`KismetMathLibrary.MakeVector` (.x _boxextent) 0.0 (.z _boxextent)))) (`KismetMathLibrary.MakeRotator` 0.0 0.0 (select `bool` (`KismetMathLibrary.RandomBool`) :`false` 90.0 :`true` 270.0 :!type "Float (single-precision)")) (* (`KismetMathLibrary.MakeVector` (`KismetMathLibrary.RandomFloatInRange` 0.8 1.0) (`KismetMathLibrary.RandomFloatInRange` 0.8 1.0) (`KismetMathLibrary.RandomFloatInRange` 0.8 1.0)) (`KismetMathLibrary.RandomFloatInRange` _scalesize_x _scalesize_y))) "AlwaysSpawn" "OverrideRootScale" null (`self.Speed`) (`self.Material`) null))
  (return _returnvalue))

(fn `UserConstructionScript`)