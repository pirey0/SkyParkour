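; Interactable structure that registers with BP_DesignGameMode on BeginPlay and can be activated once as a findable world objective.
; Interacting plays an optional cutscene through its camera, reports the find to the game mode and removes the UI trigger.
; After timed delays it fires a light pillar sound and point light, toggles a component's visibility, then shows the game mode's discovery text in a HUD widget faded by a timeline.
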(event `self.ReceiveBeginPlay`
  (bind _asbp_design_game_mode (cast `/Game/Blueprints/DesignPrototype/BP_DesignGameMode` (`GameplayStatics.GetGameMode`)))
  (`/Game/Blueprints/DesignPrototype/BP_DesignGameMode.RegisterInteractableStructure` _asbp_design_game_mode))

(event `/Game/Blueprints/Interface/BPI_Interact.Interact`
  (params (Actor :type "Actor Object Reference"))
  (bind _uitrigger (`self.UITrigger`))
  (bind _cutscene (`self.Cutscene`))
  (if (not (`self.acticated`))
    (set `self.acticated` true)
    (`|ExecutionSequence`
      (:`then_0`
        (`/Engine/EditorBlueprintResources/StandardMacros.IsValid` _cutscene
          (:`Is Valid`
            (`MovieSceneSequencePlayer.Play` (`LevelSequenceActor.SequencePlayer` _cutscene))
            (`PlayerController.SetViewTargetWithBlend` (`GameplayStatics.GetPlayerController` 0) (`self.CutsceneCamera`) 0.0 "VTBlend_Linear" 0.0 false))))
      (:`then_1`
        (bind _asbp_design_game_mode (cast `/Game/Blueprints/DesignPrototype/BP_DesignGameMode` (`GameplayStatics.GetGameMode`))
          (:`then`
            (`/Game/Blueprints/DesignPrototype/BP_DesignGameMode.FindInteractableStructure` _asbp_design_game_mode))
          (:`CastFailed`
            (`GameplayStatics.PlaySound2D` null 1.0 1.0 0.0 null null))))
      (:`then_2`
        (`KismetSystemLibrary.Delay` (`self.Delay`))
        (`GameplayStatics.PlaySoundAtLocation` "/Game/Blueprints/Lucas/lightPillarSound.lightPillarSound" (`self.K2_GetActorLocation`) (struct) 1.0 1.0 0.0 null null null)
        (`LightComponent.SetIntensity` (`self.PointLight`) (`self.Intensity`))
        (`KismetSystemLibrary.Delay` 5.2)
        (`SceneComponent.ToggleVisibility` (`self.ewew`) false)
        (bind _displaytext (`/Game/Blueprints/DesignPrototype/BP_DesignGameMode.GetInteractableStructureOnFindText` _asbp_design_game_mode))
        (bind _returnvalue (`|CreateWidget` "/Game/UI/WBP_InteractableStructure_HUD.WBP_InteractableStructure_HUD_C" null _displaytext))
        (`UserWidget.AddToViewport` _returnvalue 0)
        (bind (_direction _opacity) (`Timeline|TL_FadeInAndOut` :`NewTime` 1.0)
          (:`Update`
            (`Widget.SetRenderOpacity` _returnvalue _opacity))
          (:`Finished`
            (`Widget.RemoveFromParent` _returnvalue))))
      (:`then_3`
        (`/Engine/EditorBlueprintResources/StandardMacros.IsValid` _uitrigger
          (:`Is Valid`
            (`ActorComponent.K2_DestroyComponent` _uitrigger)))))))

(fn `UserConstructionScript`)