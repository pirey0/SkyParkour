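; BP_Boids_Path is a design prototype boids actor that feeds its flock a looping series of targets from a spline path.
; Each tick it compares the boid center to the current target and advances to the next spline point within a set distance, wrapping at the end.
; It draws a debug sphere at the center, prints target changes, and sizes its Sphere component from MRadius at construction.
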(event `self.ReceiveBeginPlay`
  (set `self.m_Target` (`SplineComponent.GetLocationAtSplinePoint` (`self.PathSpline`) 0 "World")))

(event `self.ReceiveTick`
  (params (DeltaSeconds :type "Float (single-precision)"))
  (`KismetSystemLibrary.DrawDebugSphere` (+ (`self.K2_GetActorLocation`) (`self.m_BoidCenter`)) 100.0 12 (struct :`R` 1.0 :`B` 0.12231 :`A` 1.0) 0.1)
  (if (< (`KismetMathLibrary.Vector_Distance` (`self.m_Target`) (+ (`self.K2_GetActorLocation`) (`self.m_BoidCenter`))) (`self.DistanceToNextTarget`))
    (`/Engine/EditorBlueprintResources/StandardMacros.IncrementInt` (`self.currentSplineId`)
      (:`  `
        (if (>= (`self.currentSplineId`) (`SplineComponent.GetNumberOfSplinePoints` (`self.PathSpline`)))
          (set `self.currentSplineId` 0))
        (bind _output_get (set `self.m_Target` (`SplineComponent.GetLocationAtSplinePoint` (`self.PathSpline`) (`self.currentSplineId`) "World")))
        (`KismetSystemLibrary.PrintString` (`KismetStringLibrary.Concat_StrStr` "New Target: " (`KismetStringLibrary.Conv_VectorToString` _output_get)) true false (struct :`R` 1.0 :`G` 0.087957 :`A` 1.0))))))

(fn `UserConstructionScript`
  (`SphereComponent.SetSphereRadius` (`self.Sphere`) (`KismetMathLibrary.Conv_IntToDouble` (`self.m_Radius`)) false))