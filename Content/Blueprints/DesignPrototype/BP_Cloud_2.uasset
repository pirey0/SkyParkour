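; BP_Cloud_2 is a prototype cloud actor that randomizes the look of three static mesh components and drifts the first.
; On BeginPlay each component gets a random mesh from CloudMeshes and the MaterialInst material.
; Tick moves StaticMesh along relative Y by Speed scaled by delta time.
; The offsets for StaticMesh2 and StaticMesh3 are multiplied by zero, so Tick adds no movement to them.
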(event `self.ReceiveBeginPlay`
  (bind _staticmesh3 (`self.StaticMesh3`))
  (bind _cloudmeshes (`self.CloudMeshes`))
  (bind _staticmesh2 (`self.StaticMesh2`))
  (bind _cloudmeshes_2 (`self.CloudMeshes`))
  (bind _cloudmeshes_3 (`self.CloudMeshes`))
  (`StaticMeshComponent.SetStaticMesh` (`self.StaticMesh`) (`|GetArrayItem` _cloudmeshes (`KismetMathLibrary.RandomIntegerInRange` 0 (- (`KismetArrayLibrary.Array_Length` _cloudmeshes) 1))))
  (`PrimitiveComponent.SetMaterial` (`self.StaticMesh`) 0 (`self.MaterialInst`))
  (`PrimitiveComponent.SetMaterial` (`self.StaticMesh`) 0 (`self.MaterialInst`))
  (`StaticMeshComponent.SetStaticMesh` _staticmesh2 (`|GetArrayItem` _cloudmeshes_2 (`KismetMathLibrary.RandomIntegerInRange` 0 (- (`KismetArrayLibrary.Array_Length` _cloudmeshes_2) 1))))
  (`PrimitiveComponent.SetMaterial` _staticmesh2 0 (`self.MaterialInst`))
  (`StaticMeshComponent.SetStaticMesh` _staticmesh3 (`|GetArrayItem` _cloudmeshes_3 (`KismetMathLibrary.RandomIntegerInRange` 0 (- (`KismetArrayLibrary.Array_Length` _cloudmeshes_3) 1))))
  (`PrimitiveComponent.SetMaterial` _staticmesh3 0 (`self.MaterialInst`)))

(event `self.ReceiveTick`
  (params (DeltaSeconds :type "Float (single-precision)"))
  (`SceneComponent.K2_AddRelativeLocation` (`self.StaticMesh`) (* (`KismetMathLibrary.MakeVector` 0.0 (`self.Speed`)) DeltaSeconds) false false)
  (`SceneComponent.K2_AddRelativeLocation` (`self.StaticMesh2`) (* (`KismetMathLibrary.MakeVector` 0.0 (`self.Speed`)) 0.0) false false)
  (`SceneComponent.K2_AddRelativeLocation` (`self.StaticMesh3`) (* (`KismetMathLibrary.MakeVector` 0.0 (`self.Speed`)) 0.0) false false))

(fn `UserConstructionScript`)