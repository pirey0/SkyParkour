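; Boids flocking prototype actor that simulates a swarm of mesh instances, spawned at random within a radius on construction.
; Each Tick steers velocities by brute-force all-pairs separation, flock-wide average alignment and cohesion, and a pull toward a Target re-randomized every ten seconds.
; Speeds are clamped, then positions and velocity-facing rotations are integrated in arrays and pushed in one batched instance update, with optional debug drawing.
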(event `self.ReceiveBeginPlay`
  (`KismetSystemLibrary.RetriggerableDelay` 10.0 :!label _label)
  (set `self.Target` (* (`KismetMathLibrary.MakeVector` (`KismetMathLibrary.RandomFloat`) (`KismetMathLibrary.RandomFloat`) (`KismetMathLibrary.RandomFloat`)) 5000.0))
  (goto _label))

(event `self.ReceiveTick`
  (params (DeltaSeconds :type "Float (single-precision)"))
  (`self.UpdateBoids` DeltaSeconds))

(fn `CalculateAllignment`
  (returns (All :type "Vector Structure"))
  (locals (Allignment :type "Vector Structure"))
  (bind _velocities (`self.Velocities`))
  (for _array_element _velocities
    (set `local.Allignment` (+ (`local.Allignment`) _array_element)))
  (return (/ (`local.Allignment`) (`KismetArrayLibrary.Array_Length` _velocities))))

(fn `CalculateCenter`
  (returns (Location :type "Vector Structure"))
  (locals (LocVal :type "Vector Structure"))
  (bind _transforms (`self.Transforms`))
  (for _array_element _transforms
    (set `local.LocVal` (+ (`local.LocVal`) (.location _array_element))))
  (return (/ (`local.LocVal`) (`KismetMathLibrary.Conv_IntToDouble` (`KismetArrayLibrary.Array_Length` _transforms)))))

(fn `CalculateSeparation`
  (params (Center :type "Vector Structure"))
  (returns (Sep :type "Vector Structure"))
  (locals (Separation :type "Vector Structure"))
  (for _array_element (`self.Transforms`)
    (bind _returnvalue (- (.location _array_element) Center))
    (set `local.Separation` (- (`local.Separation`) (/ _returnvalue (`KismetMathLibrary.VSizeSquared` _returnvalue)))))
  (return (`local.Separation`)))

(fn `DebugDraw`
  (for (_array_element _array_index) (`self.Transforms`)
    (bind _returnvalue (+ (`self.K2_GetActorLocation`) (.location _array_element)))
    (`KismetSystemLibrary.DrawDebugArrow` _returnvalue (+ _returnvalue (`|GetArrayItem` (`self.Velocities`) _array_index)) 15.0 (struct :`G` 0.194179 :`B` 0.625 :`A` 1.0) 0.0 5.0)
    (`KismetSystemLibrary.DrawDebugSphere` _returnvalue 100.0 12 (struct :`R` 1.0 :`G` 1.0 :`B` 1.0 :`A` 0.2))
    (`KismetSystemLibrary.DrawDebugSphere` _returnvalue 100.0 12 (struct :`R` 1.0 :`A` 0.2))))

(fn `SpawnBoids`
  (bind _returnvalue (`KismetMathLibrary.MakeTransform` (* (* (`KismetMathLibrary.RandomUnitVector`) (`KismetMathLibrary.MapRangeClamped` (`KismetMathLibrary.RandomFloat`) 0.0 1.0 0.2 1.0)) (`self.Radius`)) (`KismetMathLibrary.RandomRotator` false) (`KismetMathLibrary.Conv_DoubleToVector` (+ (`KismetMathLibrary.RandomFloat`) 0.5))))
  (`InstancedStaticMeshComponent.ClearInstances` (`self.Boids`))
  (`KismetArrayLibrary.Array_Clear` (`self.Transforms`))
  (`KismetArrayLibrary.Array_Clear` (`self.Velocities`))
  (for _ (range (+ (`self.Amount`) 1))
    (`KismetArrayLibrary.Array_Add` (`self.Transforms`) _returnvalue)
    (`InstancedStaticMeshComponent.AddInstance` (`self.Boids`) _returnvalue)
    (`KismetArrayLibrary.Array_Add` (`self.Velocities`) (* (`KismetMathLibrary.GetForwardVector` (.rotation _returnvalue)) (`self.StartSpeed`)))))

(fn `UpdateBoids`
  (params (DeltaTime :type "Float (double-precision)"))
  (`self.UpdateVelocities` DeltaTime)
  (`self.UpdatePositions` DeltaTime)
  (`InstancedStaticMeshComponent.BatchUpdateInstancesTransforms` (`self.Boids`) 0 (`self.Transforms`) false false false)
  (if (`self.Debug`)
    (`self.DebugDraw`)))

(fn `UpdatePositions`
  (params (DeltaTime :type "Float (double-precision)"))
  (for (_array_element _array_index) (`self.Transforms`)
    (bind _output (`|GetArrayItem` (`self.Velocities`) _array_index))
    (`KismetArrayLibrary.Array_Set` (`self.Transforms`) _array_index (`KismetMathLibrary.MakeTransform` (+ (.location _array_element) (* _output DeltaTime)) (`KismetMathLibrary.MakeRotFromZ` (`KismetMathLibrary.Normal` _output)) (.scale _array_element)))))

(fn `UpdateVelocities`
  (params (DeltaTime :type "Float (double-precision)"))
  (locals (Center :type "Vector Structure") (Alignment :type "Vector Structure") (Separation :type "Vector Structure") (Position :type "Vector Structure") (Index :type Integer) (NewLocalVar_0 :type "Float (double-precision)"))
  (bind _location (`self.CalculateCenter`))
  (set `local.Center` _location)
  (bind _all (`self.CalculateAllignment`))
  (set `local.Alignment` _all)
  (for (_array_element _array_index) (`self.Transforms`)
    (set `local.Index` _array_index)
    (set `local.Position` (.location _array_element))
    (bind _sep (`self.CalculateSeparation` (`local.Position`)))
    (set `local.Separation` _sep)
    (`KismetArrayLibrary.Array_Set` (`self.Velocities`) (`local.Index`) (`KismetMathLibrary.ClampVectorSize` (+ (* (+ (* (`local.Separation`) (`self.SeparationMult`)) (* (`local.Alignment`) (`self.AlignmentMult`)) (* (- (`local.Center`) (`local.Position`)) (`self.CohesionMult`)) (* (`self.Norm` (- (`self.Target`) (+ (`self.K2_GetActorLocation`) (`local.Position`)))) (`self.CenterMult`))) (`local.DeltaTime`)) (`|GetArrayItem` (`self.Velocities`) (`local.Index`))) (`self.MinSpeed`) (`self.TopSpeed`)))))

(fn `UserConstructionScript`
  (`self.SpawnBoids`))