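; Prototype crafting zone actor that turns items placed inside it into a new item.
; It tracks overlapping actors and, on each new overlap, counts those whose class exactly matches the required one.
; Once the count reaches the required amount, it destroys all matches, spawns the result at its own location, activates a particle effect and plays a clank sound.
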(event `self.ReceiveBeginPlay`
  (`ActorComponent.Deactivate` (`self.ParticleSystem1`)))

(event `self.ReceiveActorBeginOverlap`
  (params (OtherActor :type "Actor Object Reference"))
  (bind _overlapping (`self.Overlapping`))
  (`KismetArrayLibrary.Array_Add` _overlapping OtherActor)
  (`KismetArrayLibrary.Array_Clear` (`self.LocalSet`))
  (set `self.LocalCounter` 0)
  (for _array_element _overlapping
    (if (== (`GameplayStatics.GetObjectClass` _array_element) (`self.Required`))
      (`/Engine/EditorBlueprintResources/StandardMacros.IncrementInt` (`self.LocalCounter`)
        (:`  `
          (`KismetArrayLibrary.Array_Add` (`self.LocalSet`) _array_element)))))
  (if (>= (`self.LocalCounter`) (`self.RequiredAmount`))
    (for _array_element_2 (`self.LocalSet`)
      (`KismetArrayLibrary.Array_RemoveItem` (`self.Overlapping`) _array_element_2)
      (`self.K2_DestroyActor` _array_element_2))
    (`|SpawnActorFromClass` (`self.SpawnedItem`) (`KismetMathLibrary.MakeTransform` (`self.K2_GetActorLocation`)) "AlwaysSpawn" "OverrideRootScale" null null)
    (`ActorComponent.Activate` (`self.ParticleSystem1`) true)
    (`GameplayStatics.PlaySoundAtLocation` "/Game/Blueprints/DesignPrototype/clank.clank" (`self.K2_GetActorLocation`) (struct) 3.0 1.0 0.0 null null null)))

(event `self.ReceiveActorEndOverlap`
  (params (OtherActor :type "Actor Object Reference"))
  (`KismetArrayLibrary.Array_RemoveItem` (`self.Overlapping`) OtherActor))

(fn `UserConstructionScript`)