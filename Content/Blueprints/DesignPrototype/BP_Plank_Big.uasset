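; BP_Plank_Big is a prototype big plank prop that characters can pick up and drop.
; Pickup snaps the Collider to the character mesh's pickup_r socket with physics and collision off; Drop detaches it and restores both.
; It also reports the Collider as the component to pick up and supplies a pickup overlay type.
; Interact is an empty stub.
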(event `/Game/Blueprints/Interface/BPI_Interact.Interact`
  (params (Actor :type "Actor Object Reference"))
  ;[1 1 1] Interact
)

(event `Pickup_1`
  (params (InteractingActor :type "Actor Object Reference"))
  (bind _collider (`self.collider`))
  ;[1 1 1] Pickup
  (bind _ascharacter (cast `Character` InteractingActor))
  (`SceneComponent.K2_AttachToComponent` (`self.collider`) (`Character.Mesh` _ascharacter) "pickup_r" "SnapToTarget" "SnapToTarget" "KeepRelative" true)
  (`PrimitiveComponent.SetSimulatePhysics` _collider false)
  (`PrimitiveComponent.SetCollisionEnabled` _collider "NoCollision"))

(event `Drop_1`
  (bind _collider (`self.collider`))
  ;[1 1 1] Drop
  (`SceneComponent.K2_DetachFromComponent` (`self.collider`) "KeepWorld" "KeepWorld" "KeepWorld" true)
  (`PrimitiveComponent.SetSimulatePhysics` _collider true)
  (`PrimitiveComponent.SetCollisionEnabled` _collider "QueryAndPhysics"))

(fn `GetComponentToPickUp`
  (returns (Comp :type "BoxComponent Object Reference"))
  (return (`self.collider`)))

(fn `GetPickupOverlayType`
  (returns (Type :type "/Game/AdvancedLocomotionV4/Data/Enums/ALS_OverlayState Enum"))
  (return "NewEnumerator11"))

(fn `UserConstructionScript`)