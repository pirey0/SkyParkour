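; BP_WalkingGolem is a scripted golem actor that walks from its placed position to a target point, then disappears.
; It starts hidden at BeginPlay until OnTriggeron reveals it and loops its walking animation.
; A Move timeline lerps the actor from its start location to the TargetPos component's world location with teleporting moves, then destroys it.
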(event `self.ReceiveBeginPlay`
  (`self.HideGolem` true))

(event `HideGolem`
  (params (hide :type Boolean))
  (bind _returnvalue (not hide))
  (`SceneComponent.SetVisibility` (`self.SkeletalMeshComponent`) _returnvalue false)
  (if _returnvalue
    (`SkeletalMeshComponent.PlayAnimation` (`self.SkeletalMeshComponent`) "/Game/Environment/09_TempAssets/Max/AztecGolem/walking_Anim.walking_Anim" true)))

(event `/Game/Blueprints/Lucas/Lightsystem/BPI_Triggerable.OnTriggerOn`
  (`self.StartWalking`))

(event `StartWalking`
  (`self.HideGolem` false)
  (`|ExecutionSequence`
    (:`then_0`
      (bind _output_get (set `self.targetPosVector` (`SceneComponent.K2_GetComponentLocation` (`self.targetPos`)))))
    (:`then_1`
      (bind _output_get_2 (set `self.startPosVector` (`self.K2_GetActorLocation`))))
    (:`then_2`
      (bind (_direction _translate) (`Timeline|move`)
        (:`Update`
          (`self.K2_SetActorLocation` (`KismetMathLibrary.VLerp` _output_get_2 _output_get _translate) false true))
        (:`Finished`
          (`self.K2_DestroyActor`))))))

(fn `UserConstructionScript`)