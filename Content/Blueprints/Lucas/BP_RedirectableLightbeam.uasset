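; Lightbeam actor, apparently an unfinished prototype, that line-traces on the Visibility channel every Tick and prints the hit distance.
; The trace ends at the raw forward vector, not an offset from the actor, and stores its end point and distance.
; UpdateLightbeamLength repositions and scales the Beam component from those values, but nothing executes it.
; No redirection logic is present, and MaxLength is unused.
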(event `self.ReceiveTick`
  (params (DeltaSeconds :type "Float (single-precision)"))
  (bind _outhit (`KismetSystemLibrary.LineTraceSingle` :`Start` (`self.K2_GetActorLocation`) :`End` (`self.GetActorForwardVector`) :`TraceChannel` "TraceTypeQuery1" :`DrawDebugType` "ForDuration"))
  (bind (_bblockinghit _binitialoverlap _time _distance _location _impactpoint _normal _impactnormal _physmat _hitactor _hitcomponent _hitbonename _hititem _faceindex _tracestart _traceend) (`GameplayStatics.BreakHitResult` _outhit))
  (set `self.End` _traceend)
  (set `self.length` _distance)
  (`KismetSystemLibrary.PrintString` (`KismetStringLibrary.Conv_DoubleToString` _distance)))

(fn `UpdateLightbeamLength`
  (bind _returnvalue (`self.K2_GetActorLocation`))
  (bind _beamwidth (`self.BeamWidth`))
  ;[1 1 1] Position
  (`SceneComponent.K2_SetWorldLocation` (`self.beam`) (+ _returnvalue (/ (- (`self.End`) _returnvalue) 0.5)) false true)
  ;[1 1 1] Scale
  (`SceneComponent.SetRelativeScale3D` (`self.beam`) (`KismetMathLibrary.MakeVector` _beamwidth _beamwidth (`self.length`))))

(fn `UserConstructionScript`)