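; BP_DesignGameMode is a game mode that tracks how many interactable structures have been found out of the total registered.
; RegisterInteractableStructure increments the maximum count, and FindInteractableStructure increments the activated count.
; GetInteractableStructureOnFindText formats both counters as an "(activated/max)" text.
; The event graph and construction script hold no logic.
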(fn `FindInteractableStructure`
  (set `self.numberOfStructuresActivated` (+ (`self.numberOfStructuresActivated`) 1)))

(fn `GetInteractableStructureOnFindText`
  (returns (DisplayText :type Text))
  (return (`KismetTextLibrary.Conv_StringToText` (`KismetStringLibrary.Concat_StrStr` (`KismetStringLibrary.Concat_StrStr` (`KismetStringLibrary.Concat_StrStr` (`KismetStringLibrary.Concat_StrStr` "( " (`KismetStringLibrary.Conv_IntToString` (`self.numberOfStructuresActivated`))) " / ") (`KismetStringLibrary.Conv_IntToString` (`self.numberOfStructuresMax`))) " )"))))

(fn `RegisterInteractableStructure`
  (set `self.numberOfStructuresMax` (+ (`self.numberOfStructuresMax`) 1)))

(fn `UserConstructionScript`)