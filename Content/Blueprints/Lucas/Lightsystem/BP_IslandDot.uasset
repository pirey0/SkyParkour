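; BP_IslandDot is a light system actor with a dot that appears after enough activations and feeds a linked light cannon.
; The dot starts hidden, and each Triggeron event increments an activation counter.
; At or above the required count, it waits a configurable delay, shows the dot and calls InsertShard on the cannon if valid.
; The counter never resets, so later triggers can repeat that sequence.
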(event `self.ReceiveBeginPlay`
  (`SceneComponent.SetVisibility` (`self.dot`) false false))

(event `/Game/Blueprints/Lucas/Lightsystem/BPI_Triggerable.OnTriggerOn`
  (bind _lightcanon (`self.lightcanon`))
  (bind _output_get (set `self.amountOfAcivations` (+ (`self.amountOfAcivations`) 1)))
  (if (>= _output_get (`self.amountOfAcivationsNeeded`))
    (`KismetSystemLibrary.Delay` (`self.delay`))
    (`SceneComponent.SetVisibility` (`self.dot`) true false)
    (`/Engine/EditorBlueprintResources/StandardMacros.IsValid` _lightcanon
      (:`Is Valid`
        (`/Game/Blueprints/Lucas/Lightsystem/BP_FinalPlatform.insertShard` _lightcanon)))))

(fn `UserConstructionScript`)