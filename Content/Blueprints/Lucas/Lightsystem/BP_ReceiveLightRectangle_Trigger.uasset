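; BP_ReceiveLightRectangle_Trigger is a rectangular light-receiver Blueprint in the Lightsystem whose Frame component appears when triggered.
; On BeginPlay it runs the parent logic, then hides the Frame unless FrameVisibleOnSpawn is set.
; The OnTriggeron event makes the Frame visible again, and no handler here hides it afterward.
; GetCenter returns a zero vector, and the construction script only calls its parent.
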(event `self.ReceiveBeginPlay`
  (`parent.ReceiveBeginPlay`)
  (if (not (`self.frameVisibleOnSpawn`))
    (`SceneComponent.SetVisibility` (`self.frame`) false false)))

(event `/Game/Blueprints/Lucas/Lightsystem/BPI_Triggerable.OnTriggerOn`
  (`SceneComponent.SetVisibility` (`self.frame`) true false))

(fn `GetCenter`
  (returns (NewParam :type "Vector Structure"))
  (return (0.0 0.0 0.0)))

(fn `UserConstructionScript`
  (`parent.UserConstructionScript`))