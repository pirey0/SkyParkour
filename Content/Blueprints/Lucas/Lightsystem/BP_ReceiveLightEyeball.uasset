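; BP_ReceiveLightEyeball is an eyeball-themed actor in the light system that shows light-receiving progress as emissive glow.
; On BeginPlay it runs the parent logic, creates a dynamic material on the Receiver component and resets the visualization to zero.
; Its UpdateVisualiazion event turns a progression value into the material's Emissive_Mult parameter through a scaled cubic curve, so brightness ramps up steeply.
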(event `self.ReceiveBeginPlay`
  (bind _receiver (`self.receiver`))
  (`parent.ReceiveBeginPlay`)
  (bind _returnvalue (`PrimitiveComponent.CreateDynamicMaterialInstance` _receiver 0 (`PrimitiveComponent.GetMaterial` _receiver 0) "None"))
  (set `self.material` _returnvalue)
  (`self.UpdateVisualiazion` 0.0))

(event `self.UpdateVisualiazion`
  (params (progression :type "Float (single-precision)"))
  (bind _material (`self.material`))
  (`/Engine/EditorBlueprintResources/StandardMacros.IsValid` _material
    (:`Is Valid`
      (`MaterialInstanceDynamic.SetScalarParameterValue` _material "Emissive_Mult" (`KismetMathLibrary.MultiplyMultiply_FloatFloat` (* progression 3.0) 3.0)))))

(fn `UserConstructionScript`
  (`parent.UserConstructionScript`))