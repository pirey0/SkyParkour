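; Triggerable moving element, such as a puzzle door, that slides between two positions when switched on or off.
; On BeginPlay it stores the element's start position and the target from a placeholder component, which it then destroys.
; Trigger on plays a timeline that blends the relative location toward the target, and trigger off reverses it.
; Both play the PuzzleMovingDoor sound from DT_SoundLib at the actor's location.
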(event `self.ReceiveBeginPlay`
  (bind _positiontomoveto (`self.positionToMoveTo`))
  ;[1 1 1] Define Locations
  (set `self.startPos` (`SceneComponent.RelativeLocation` (`self.elementToMove`)))
  (set `self.targetPos` (`SceneComponent.RelativeLocation` _positiontomoveto))
  (`ActorComponent.K2_DestroyComponent` _positiontomoveto))

(event `/Game/Blueprints/Lucas/Lightsystem/BPI_Triggerable.OnTriggerOn`
  (`|ExecutionSequence`
    (:`then_0`
      ;[1 1 1] Open / Close Timeline
      (bind (_direction _amount) (`Timeline|moving` :!label _label)
        (:`Update`
          (`|ExecutionSequence`
            (:`then_0`
              (bind _blended_vector (`self.Blend Between Vectors` (`self.targetPos`) (`self.startPos`) _amount))
              (`SceneComponent.K2_SetRelativeLocation` (`self.elementToMove`) _blended_vector false true))))))
    (:`then_1`
      ;[1 1 1] Play Sound
      (bind _returnvalue (`|GetDataTableRow` "/Game/Blueprints/Datatables/DT_SoundLib.DT_SoundLib" "PuzzleMovingDoor" :!label _label_2)
        (:`then`
          (`GameplayStatics.PlaySoundAtLocation` (break `/Game/Blueprints/Datatables/S_SoundData` _returnvalue) (`self.K2_GetActorLocation`) (struct) 1.0 1.0 0.0 null null null))))))

(event `/Game/Blueprints/Lucas/Lightsystem/BPI_Triggerable.OnTriggerOff`
  (if true
    (`|ExecutionSequence`
      (:`then_0`
        (goto _label :!via `Reverse`))
      (:`then_1`
        (goto _label_2)))))

(fn `Blend Between Vectors`
  (params (`vector 1` :type "Vector Structure") (`vector 2` :type "Vector Structure") (blendAmount :type "Float (double-precision)"))
  (returns (`blended Vector` :type "Vector Structure"))
  (return (+ (* `vector 1` blendAmount) (* `vector 2` (- 1.0 blendAmount)))))

(fn `UserConstructionScript`)