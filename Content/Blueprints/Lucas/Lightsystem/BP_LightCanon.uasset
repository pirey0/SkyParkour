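; BP_LightCanon is a light-system actor that counts inserted shards and opens its platform once the required number is reached.
; At the threshold, it triggers its additional visualization objects through BPI_Triggerable and plays a timeline that slides two platform halves to their target components' positions.
; When that finishes, an elevator timeline lowers the center piece, with all movement lerped from start locations cached at BeginPlay.
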(event `self.ReceiveBeginPlay`
  (`|ExecutionSequence`
    (:`then_0`
      (set `self.platformHalfPiece1_startLocation` (`SceneComponent.RelativeLocation` (`self.platformHalfPiece1`))))
    (:`then_1`
      (set `self.platformHalfPiece2_startLocation` (`SceneComponent.RelativeLocation` (`self.platformHalfPiece2`))))
    (:`then_2`
      (set `self.platformCenterPiece_startLocation` (`SceneComponent.RelativeLocation` (`self.platformCenterPiece`))))))

(event `insertShard`
  (bind _numberofshards (`self.AddShard`))
  (if (>= _numberofshards (`self.numberOfShardsNeeded`))
    (`|ExecutionSequence`
      (:`then_0`
        ;[1 1 1] Enable Additional Visualizations
        (for _array_element (`self.AdditionalVisualizations`)
          (if (`KismetSystemLibrary.DoesImplementInterface` _array_element "/Game/Blueprints/Lucas/Lightsystem/BPI_Triggerable.BPI_Triggerable_C")
            (message `/Game/Blueprints/Lucas/Lightsystem/BPI_Triggerable.OnTriggerOn` _array_element))))
      (:`then_1`
        ;[1 1 1] opening pieces
        (bind (_direction _open) (`Timeline|piecesOpening`)
          (:`Update`
            (`|ExecutionSequence`
              (:`then_0`
                (`SceneComponent.K2_SetRelativeLocation` (`self.platformHalfPiece1`) (`KismetMathLibrary.VLerp` (`self.platformHalfPiece1_startLocation`) (`SceneComponent.RelativeLocation` (`self.platformHalfPiece1_target`)) _open) false true))
              (:`then_1`
                (`SceneComponent.K2_SetRelativeLocation` (`self.platformHalfPiece2`) (`KismetMathLibrary.VLerp` (`self.platformHalfPiece2_startLocation`) (`SceneComponent.RelativeLocation` (`self.platformHalfPiece2_target`)) _open) false true))))
          (:`Finished`
            ;[1 1 1] ElevatorMoveDown
            (bind (_direction_2 _move_down) (`Timeline|elevator`)
              (:`Update`
                (`SceneComponent.K2_SetRelativeLocation` (`self.platformCenterPiece`) (`KismetMathLibrary.VLerp` (`self.platformCenterPiece_startLocation`) (`SceneComponent.RelativeLocation` (`self.platformCenterPiece_target`)) _move_down) false true)))))))))

(fn `AddShard`
  (returns (numberOfShards :type Integer))
  (bind _output_get (set `self.numberOfShards` (+ (`self.numberOfShards`) 1)))
  (return _output_get))

(fn `UserConstructionScript`
  (`parent.UserConstructionScript`))