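; Final platform that shows collected shards and opens into a descending elevator once enough are gathered.
; Each game mode CollectShard event fires a cutscene camera, then increments the count and fades in a shard with an emissive glow.
; A later overlap opens it once: timelines slide the halves apart and lower the center toward target components.
; It also triggers extra visuals and a glide camera via BPI_Triggerable, with temporary anti-fall collision.
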(event `self.ReceiveBeginPlay`
  (`|ExecutionSequence`
    (:`then_0`
      ;[1 1 1] save locations for animations
      (set `self.platformHalfPiece1_startLocation` (`SceneComponent.RelativeLocation` (`self.platformHalfPiece1`))))
    (:`then_1`
      (set `self.platformHalfPiece2_startLocation` (`SceneComponent.RelativeLocation` (`self.platformHalfPiece2`))))
    (:`then_2`
      (set `self.platformCenterPiece_startLocation` (`SceneComponent.RelativeLocation` (`self.platformCenterPiece`))))
    (:`then_3`
      (`SceneComponent.SetVisibility` (`self.platformCenterPiece_target`) false false))
    (:`then_4`
      ;[1 1 1] Bind Event
      (bind _asbp_design_game_mode (cast `/Game/Blueprints/DesignPrototype/BP_DesignGameMode` (`GameplayStatics.GetGameMode`)))
      (add `/Game/Blueprints/DesignPrototype/BP_DesignGameMode.CollectShard` _asbp_design_game_mode (delegate `CollectShard_Event`)))
    (:`then_5`
      (`PrimitiveComponent.SetCollisionEnabled` (`self.stopFallof`) "NoCollision"))))

(event `CollectShard_Event`
  ;[1 1 1] Add Shard Event
  (`/Game/Blueprints/Lucas/Lightsystem/BPI_Triggerable.OnTriggerOn` (`self.CutsceneCam`))
  (`KismetSystemLibrary.Delay` 0.5)
  (bind _output_get (set `self.numberOfShards` (+ (`self.numberOfShards`) 1)))
  (`|ExecutionSequence`
    (:`then_0`
      (`GameplayStatics.PlaySoundAtLocation` "/Game/SFX/Puzzle/bongwav2_long.bongwav2_long" (`self.K2_GetActorLocation`) (struct) 1.0 1.0 0.0 null null null))
    (:`then_1`
      (bind _shard (`self.GetShardByInt` _output_get))
      (bind (_direction _dissolve) (`Timeline|FadeIn`)
        (:`Update`
          (`/Game/Blueprints/Lucas/finalPlatform/BP_collectedShard.SetDissolve` _shard _dissolve))
        (:`Finished`
          ;[1 1 1] Set shard emissive
          (bind _returnvalue (`PrimitiveComponent.CreateDynamicMaterialInstance` _shard 0 (`PrimitiveComponent.GetMaterial` _shard 0) "None"))
          (bind (_direction_2 _emissive) (`Timeline|SetEmissive`)
            (:`Update`
              (`MaterialInstanceDynamic.SetScalarParameterValue` _returnvalue "EmissiveMult" _emissive))))))))

(event `self.ReceiveActorBeginOverlap`
  (params (OtherActor :type "Actor Object Reference"))
  (bind _glidingdowncam (`self.GlidingDownCam`))
  ;[1 1 1] Check For Player Enter Platform
  ;[1 1 1] All Shards collected
  (if (and (>= (`self.numberOfShards`) (`self.numberOfShardsNeeded`)) (`self.notOpen`))
    (set `self.notOpen` false)
    (`|ExecutionSequence`
      (:`then_0`
        (`PrimitiveComponent.SetCollisionEnabled` (`self.stopFallof`) "QueryAndPhysics")
        (`PrimitiveComponent.SetMaterial` (`self.platformCenterPiece`) 0 "/Game/Environment/02_Manmade/Aztek/Aztec_final_Door_emissive_INST.Aztec_final_Door_emissive_INST"))
      (:`then_1`
        ;[1 1 1] Enable Additional Visualizations
        (for _array_element (`self.AdditionalVisualizations`)
          (if (`KismetSystemLibrary.DoesImplementInterface` _array_element "/Game/Blueprints/Lucas/Lightsystem/BPI_Triggerable.BPI_Triggerable_C")
            (message `/Game/Blueprints/Lucas/Lightsystem/BPI_Triggerable.OnTriggerOn` _array_element)
            (else
              (bind _returnvalue (`self.GetComponentByClass` _array_element "/Game/Blueprints/Lucas/BP_TriggerableLightComponent.BP_TriggerableLightComponent_C"))
              (if (`KismetSystemLibrary.DoesImplementInterface` _returnvalue "/Game/Blueprints/Lucas/Lightsystem/BPI_Triggerable.BPI_Triggerable_C")
                (message `/Game/Blueprints/Lucas/Lightsystem/BPI_Triggerable.OnTriggerOn` _returnvalue))))))
      (:`then_2`
        (`|ExecutionSequence`
          (:`then_0`
            (`GameplayStatics.PlaySoundAtLocation` "/Game/Blueprints/Lucas/Sounds/platformOpening.platformOpening" (`self.K2_GetActorLocation`) (struct) 1.0 1.0 0.0 null null null))
          (:`then_1`
            ;[1 1 1] opening pieces
            (bind (_direction _open) (`Timeline|piecesOpening`)
              (:`Update`
                (`|ExecutionSequence`
                  (:`then_0`
                    (`SceneComponent.K2_SetRelativeLocation` (`self.platformHalfPiece1`) (`KismetMathLibrary.VLerp` (`self.platformHalfPiece1_startLocation`) (`SceneComponent.RelativeLocation` (`self.platformHalfPiece1_target`)) _open) false true))
                  (:`then_1`
                    (`SceneComponent.K2_SetRelativeLocation` (`self.platformHalfPiece2`) (`KismetMathLibrary.VLerp` (`self.platformHalfPiece2_startLocation`) (`SceneComponent.RelativeLocation` (`self.platformHalfPiece2_target`)) _open) false true))))
              (:`Finished`
                (if (`KismetSystemLibrary.DoesImplementInterface` _glidingdowncam "/Game/Blueprints/Lucas/Lightsystem/BPI_Triggerable.BPI_Triggerable_C")
                  (`/Game/Blueprints/Lucas/Lightsystem/BPI_Triggerable.OnTriggerOn` _glidingdowncam)))))
          (:`then_2`
            ;[1 1 1] ElevatorMoveDown
            (bind (_direction_2 _move_down) (`Timeline|elevator`)
              (:`Update`
                (`SceneComponent.K2_SetRelativeLocation` (`self.platformCenterPiece`) (`KismetMathLibrary.VLerp` (`self.platformCenterPiece_startLocation`) (`SceneComponent.RelativeLocation` (`self.platformCenterPiece_target`)) _move_down) false true))
              (:`Finished`
                (`PrimitiveComponent.SetCollisionEnabled` (`self.stopFallof`) "NoCollision")))))))))

(fn `AddShard`
  (returns (numberOfShards :type Integer)))

(fn `GetShardByInt`
  (params (int :type Integer))
  (returns (shard :type "/Game/Blueprints/Lucas/finalPlatform/BP_collectedShard Object Reference"))
  (switch `int` int
    (:`0`
      (return (`self.shardOne`)))
    (:`1`
      (return (`self.shardTwo`)))
    (:`2`
      (return (`self.shardThree`)))
    (:`3`
      (return (`self.shardFour`)))))

(fn `UserConstructionScript`
  (`parent.UserConstructionScript`))