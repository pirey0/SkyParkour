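; A decal actor for the light system, a glowing light line that turns on and off when triggered.
; On BeginPlay it creates a dynamic material instance from its decal.
; The trigger-on and trigger-off events wait a configurable delay, then play or reverse the Glow timeline, which drives the material's "progression" scalar parameter to animate the glow.
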(event `self.ReceiveBeginPlay`
  ;[1 1 1] get material for glow
  (`parent.ReceiveBeginPlay`)
  (bind _returnvalue (`DecalComponent.CreateDynamicMaterialInstance` (`self.Decal`)))
  (set `self.glowMaterial` _returnvalue))

(event `/Game/Blueprints/Lucas/Lightsystem/BPI_Triggerable.OnTriggerOn`
  ;[1 1 1] let it glow
  (`KismetSystemLibrary.Delay` (`self.delay`))
  (`/Engine/EditorBlueprintResources/StandardMacros.IsValid` (`self.glowMaterial`)
    (:`Is Valid`
      (bind (_direction _glow) (`Timeline|glow` :!label _label)
        (:`Update`
          (`MaterialInstanceDynamic.SetScalarParameterValue` (`self.glowMaterial`) "progression" _glow))))))

(event `/Game/Blueprints/Lucas/Lightsystem/BPI_Triggerable.OnTriggerOff`
  ;[1 1 1] let it glow
  (`KismetSystemLibrary.Delay` (`self.delay`))
  (`/Engine/EditorBlueprintResources/StandardMacros.IsValid` (`self.glowMaterial`)
    (:`Is Valid`
      (goto _label :!via `Reverse`))))

(fn `UserConstructionScript`)