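; BP_LightSensitiveDoor is a double door that opens while its Receiver component is lit and closes when the light leaves.
; BeginPlay caches both panels' closed positions and reads open targets from the LeftDoorOpen and RightDoorOpen components.
; LightEnter plays and LightLeave reverses the Opening timeline, which moves the panels through a linear vector blend helper.
; Both events play the same explosion sound at the door.
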(event `self.ReceiveBeginPlay`
  ;[1 1 1] Define Locations
  (set `self.LeftDoorPos` (`SceneComponent.RelativeLocation` (`self.LeftDoor`)))
  (set `self.RightDoorPos` (`SceneComponent.RelativeLocation` (`self.RightDoor`)))
  (set `self.LeftDoorTargetPos` (`SceneComponent.RelativeLocation` (`self.LeftDoorOpen`)))
  (set `self.RightDoorTargetPos` (`SceneComponent.RelativeLocation` (`self.RightDoorOpen`))))

(event `/Game/Blueprints/Lucas/Lightsystem/BPI_LightSensitiveObject.LightEnter`
  (params (ComponentThatReceivedLight :type "ActorComponent Object Reference") (lightbeam :type "/Game/Blueprints/Lucas/Lightsystem/BP_Lightbeam Object Reference"))
  ;[1 1 1] Beam enter
  (if (== ComponentThatReceivedLight (`self.receiver`))
    (`|ExecutionSequence`
      (:`then_0`
        ;[1 1 1] Open / Close Timeline
        (bind (_direction _amount) (`Timeline|Opening` :!label _label)
          (:`Update`
            (`|ExecutionSequence`
              (:`then_0`
                (bind _blended_vector (`self.BlendBetweenVectors` (`self.LeftDoorPos`) (`self.LeftDoorTargetPos`) _amount))
                (`SceneComponent.K2_SetRelativeLocation` (`self.LeftDoor`) _blended_vector false true))
              (:`then_1`
                (bind _blended_vector_2 (`self.BlendBetweenVectors` (`self.RightDoorPos`) (`self.RightDoorTargetPos`) _amount))
                (`SceneComponent.K2_SetRelativeLocation` (`self.RightDoor`) _blended_vector_2 false true))))))
      (:`then_1`
        ;[1 1 1] Play Sound
        (`GameplayStatics.PlaySoundAtLocation` "/Game/StarterContent/Audio/Explosion01.Explosion01" (`self.K2_GetActorLocation`) (struct) 1.0 1.0 0.0 null null null :!label _label_2)))))

(event `/Game/Blueprints/Lucas/Lightsystem/BPI_LightSensitiveObject.LightLeave`
  (params (ComponentThatReceivedLight :type "ActorComponent Object Reference") (lightbeam :type "/Game/Blueprints/Lucas/Lightsystem/BP_Lightbeam Object Reference"))
  ;[1 1 1] Beam leave
  (if (== ComponentThatReceivedLight (`self.receiver`))
    (`|ExecutionSequence`
      (:`then_0`
        (goto _label :!via `Reverse`))
      (:`then_1`
        (goto _label_2)))))

(fn `BlendBetweenVectors`
  (params (vector1 :type "Vector Structure") (vector2 :type "Vector Structure") (blend :type "Float (double-precision)"))
  (returns (`blended Vector` :type "Vector Structure"))
  (return (+ (* vector2 blend) (* vector1 (- 1.0 blend)))))

(fn `UserConstructionScript`)