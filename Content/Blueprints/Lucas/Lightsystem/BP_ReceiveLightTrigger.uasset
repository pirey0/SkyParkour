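; Puzzle trigger that counts light beams hitting its Receiver, or incoming on/off triggers, toward a required light total.
; After a delay, each change updates Progression and an empty UpdateVisualiazion hook.
; Crossing the threshold either way sends on/off messages to Triggerable actors through BPI_Triggerable, with DT_SoundLib sounds.
; With AutoSnap, losing player control makes the beam's source mirror adjust to hit the Receiver; AutoActivateOnStart forces a high count at BeginPlay.
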(event `self.ReceiveBeginPlay`
  (if (`self.autoActivateOnStart`)
    (set `self.amountOfLights` 99)
    (`self.Update`)))

(event `/Game/Blueprints/Lucas/Lightsystem/BPI_Triggerable.OnTriggerOn`
  (`KismetSystemLibrary.Delay` (`self.delay`) :!label _label)
  (`self.AddNewSource`)
  (`self.Update`)
  (if (< (`self.progression`) 1.0) :!label _label_2
    (bind _returnvalue (`|GetDataTableRow` "/Game/Blueprints/Datatables/DT_SoundLib.DT_SoundLib" "PuzzleMovingDoor")
      (:`then`
        (`GameplayStatics.PlaySoundAtLocation` (break `/Game/Blueprints/Datatables/S_SoundData` _returnvalue) (0.0 0.0 0.0) (struct) 1.0 1.0 0.0 null null null)))))

(event `/Game/Blueprints/Lucas/Lightsystem/BPI_LightSensitiveObject.LightEnter`
  (params (ComponentThatReceivedLight :type "ActorComponent Object Reference") (lightbeam :type "/Game/Blueprints/Lucas/Lightsystem/BP_Lightbeam Object Reference"))
  (if (and (== (`self.receiver`) ComponentThatReceivedLight) (`self.usesReceiver`))
    (set `self.hittingLightbeam` lightbeam)
    (goto _label)))

(event `/Game/Blueprints/Lucas/Lightsystem/BPI_LightSensitiveObject.LightLeave`
  (params (ComponentThatReceivedLight :type "ActorComponent Object Reference") (lightbeam :type "/Game/Blueprints/Lucas/Lightsystem/BP_Lightbeam Object Reference"))
  (if (and (== (`self.receiver`) ComponentThatReceivedLight) (`self.usesReceiver`))
    (set `self.hittingLightbeam` null)
    (`KismetSystemLibrary.Delay` (`self.delay`) :!label _label_3)
    (`self.RemoveSource`)
    (`self.Update`)
    (goto _label_2)))

(event `/Game/Blueprints/Lucas/Lightsystem/BPI_Triggerable.OnTriggerOff`
  (goto _label_3))

(event `UpdateVisualiazion`
  (params (progression :type "Float (double-precision)")))

(event `/Game/Blueprints/Lucas/Lightsystem/BPI_LightSensitiveObject.OnPlayerControlChanged`
  (params (newControlled :type Boolean))
  (bind _hittinglightbeam (`self.hittingLightbeam`))
  (bind _output_get (set `self.playerInfluenced` newControlled))
  (if (and (not _output_get) (`self.autoSnap`))
    (`/Engine/EditorBlueprintResources/StandardMacros.IsValid` _hittinglightbeam
      (:`Is Valid`
        (`/Game/Blueprints/Lucas/Lightsystem/BP_LightMirror.AdjustToHit` (`/Game/Blueprints/Lucas/Lightsystem/BP_Lightbeam.mirrorItsSpawnedBy` _hittinglightbeam) (`SceneComponent.K2_GetComponentLocation` (`self.receiver`)) _hittinglightbeam)))))

(fn `AddNewSource`
  (set `self.amountOfLights` (+ (`self.amountOfLights`) 1)))

(fn `AddTriggerable`)

(fn `RemoveSource`
  (set `self.amountOfLights` (- (`self.amountOfLights`) 1)))

(fn `Update`
  (bind _progression (`self.UpdateProgression` (`self.amountOfLights`) (`self.amountOfLightsNeeded`)))
  (`self.UpdateVisualiazion` _progression)
  (if (>= _progression 1.0)
    (if (not (`self.triggered`))
      (for _array_element (`self.Triggerable`)
        (`/Engine/EditorBlueprintResources/StandardMacros.IsValid` _array_element
          (:`Is Valid`
            (if (`KismetSystemLibrary.DoesImplementInterface` _array_element "/Game/Blueprints/Lucas/Lightsystem/BPI_Triggerable.BPI_Triggerable_C")
              (message `/Game/Blueprints/Lucas/Lightsystem/BPI_Triggerable.OnTriggerOn` _array_element)))))
      (set `self.triggered` true)
      (bind _returnvalue (`|GetDataTableRow` "/Game/Blueprints/Datatables/DT_SoundLib.DT_SoundLib" "PuzzleSuccess")
        (:`then`
          (`GameplayStatics.PlaySoundAtLocation` (break `/Game/Blueprints/Datatables/S_SoundData` _returnvalue) (0.0 0.0 0.0) (struct) 1.0 1.0 0.0 null null null))))
    (elif (`self.triggered`)
      (for _array_element_2 (`self.Triggerable`)
        (`/Engine/EditorBlueprintResources/StandardMacros.IsValid` _array_element_2
          (:`Is Valid`
            (if (`KismetSystemLibrary.DoesImplementInterface` _array_element_2 "/Game/Blueprints/Lucas/Lightsystem/BPI_Triggerable.BPI_Triggerable_C")
              (message `/Game/Blueprints/Lucas/Lightsystem/BPI_Triggerable.OnTriggerOff` _array_element_2)))))
      (set `self.triggered` false)
      (bind _returnvalue_2 (`|GetDataTableRow` "/Game/Blueprints/Datatables/DT_SoundLib.DT_SoundLib" "PuzzleCancelled")
        (:`then`
          (`GameplayStatics.PlaySoundAtLocation` (break `/Game/Blueprints/Datatables/S_SoundData` _returnvalue_2) (0.0 0.0 0.0) (struct) 1.0 1.0 0.0 null null null))))))

(fn `UpdateProgression`
  (params (current :type Integer) (max :type Integer))
  (returns (progression :type "Float (double-precision)"))
  (bind _output_get (set `self.progression` (/ (`KismetMathLibrary.Conv_IntToDouble` current) (`KismetMathLibrary.Conv_IntToDouble` max))))
  (`KismetSystemLibrary.PrintString` (`KismetStringLibrary.Concat_StrStr` (`KismetStringLibrary.Concat_StrStr` (`KismetStringLibrary.Conv_IntToString` current) " / ") (`KismetStringLibrary.Conv_IntToString` max)))
  (return _output_get))

(fn `UserConstructionScript`)