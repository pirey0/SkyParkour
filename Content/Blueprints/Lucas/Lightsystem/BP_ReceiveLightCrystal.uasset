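; BP_ReceiveLightCrystal is a light-system crystal whose emissive glow reflects a progression value.
; On BeginPlay it creates a dynamic material from the Visualization component's first material and resets the glow to zero.
; UpdateVisualiazion cubes triple the progression into the Emissive_Mult parameter for a non-linear ramp, and prints that value for debugging.
; Nothing in this graph computes progression; it only handles the visual response.
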(event `self.ReceiveBeginPlay`
  (bind _visualization (`self.visualization`))
  (`parent.ReceiveBeginPlay`)
  (bind _returnvalue (`PrimitiveComponent.CreateDynamicMaterialInstance` _visualization 0 (`PrimitiveComponent.GetMaterial` _visualization 0) "None"))
  (set `self.material` _returnvalue)
  (`self.UpdateVisualiazion` 0.0))

(event `self.UpdateVisualiazion`
  (params (progression :type "Float (single-precision)"))
  (bind _material (`self.material`))
  (bind _returnvalue (`KismetMathLibrary.MultiplyMultiply_FloatFloat` (* progression 3.0) 3.0))
  (`/Engine/EditorBlueprintResources/StandardMacros.IsValid` _material
    (:`Is Valid`
      (`MaterialInstanceDynamic.SetScalarParameterValue` _material "Emissive_Mult" _returnvalue)
      (`KismetSystemLibrary.PrintString` (`KismetStringLibrary.Conv_DoubleToString` _returnvalue)))))

(fn `UserConstructionScript`
  (`parent.UserConstructionScript`))