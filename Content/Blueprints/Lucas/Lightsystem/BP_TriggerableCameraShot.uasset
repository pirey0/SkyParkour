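; BP_TriggerableCameraShot is a cutscene camera that takes over the player's view, on BeginPlay or when triggered after five seconds of game time.
; It can be one-shot, waits a start delay, destroys an optional actor, then blends to itself and disables ALS controller input.
; Unless NotBlendBack is set, it later blends to the main camera, restores input and makes the player leave any controlled mirror.
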(event `self.ReceiveBeginPlay`
  (bind _actortodestroyontrigger (`self.actorToDestroyOnTrigger`))
  (bind _blendtime (`self.blendTime`))
  ;[1 1 1] Comment
  (if (`self.activateOnPlay`)
    ;[1 1 1] one Time activcation handling
    (if (`self.oneTime`) :!label _label
      (if (not (`self.activated`))
        (set `self.activated` true :!label _label_2)
        ;[1 1 1] Get Player Controller as reference
        (bind _asals_player_controller (cast `/Game/AdvancedLocomotionV4/Blueprints/CharacterLogic/ALS_Player_Controller` (`GameplayStatics.GetPlayerController` 0)))
        ;[1 1 1] blendIn
        (`KismetSystemLibrary.Delay` (`self.startDelay`))
        (`/Engine/EditorBlueprintResources/StandardMacros.IsValid` _actortodestroyontrigger
          (:`Is Valid`
            (`self.K2_DestroyActor` _actortodestroyontrigger))
          (:`Is Not Valid`
            _))
        (`KismetSystemLibrary.PrintString` (`KismetStringLibrary.Concat_StrStr` "show cam: " (`KismetSystemLibrary.GetDisplayName` self)))
        (`PlayerController.SetViewTargetWithBlend` _asals_player_controller self _blendtime "VTBlend_Linear" 1.0 false)
        (`/Game/AdvancedLocomotionV4/Blueprints/CharacterLogic/ALS_Player_Controller.SetInputDisabled` _asals_player_controller true)
        (if (not (`self.notBlendBack`))
          ;[1 1 1] BlendOut
          (`KismetSystemLibrary.Delay` (`self.duration`))
          (`/Game/AdvancedLocomotionV4/Blueprints/CharacterLogic/ALS_Player_Controller.BlendToMainCam` _asals_player_controller _blendtime)
          (`/Game/AdvancedLocomotionV4/Blueprints/CharacterLogic/ALS_Player_Controller.SetInputDisabled` _asals_player_controller false)
          (bind _asbp_design_game_mode (cast `/Game/Blueprints/DesignPrototype/BP_DesignGameMode` (`GameplayStatics.GetGameMode`)))
          (bind (_controllingmirror _mirror) (`/Game/Blueprints/DesignPrototype/BP_DesignGameMode.GetControllingMirror` _asbp_design_game_mode))
          (if _controllingmirror
            (`/Game/Blueprints/Lucas/Lightsystem/BP_LightMirror.LeaveMirror` _mirror))))
      (else
        (goto _label_2)))))

(event `/Game/Blueprints/Lucas/Lightsystem/BPI_Triggerable.OnTriggerOn`
  ;[1 1 1] Comment
  (if (> (`GameplayStatics.GetTimeSeconds`) 5.0)
    (goto _label)))

(fn `UserConstructionScript`)