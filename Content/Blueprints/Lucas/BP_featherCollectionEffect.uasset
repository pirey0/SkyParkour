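; Visual effect actor for feather collection, animating a ring-and-line material on a static mesh.
; On BeginPlay it creates and stores a dynamic instance of the mesh's first material.
; PlayEffect sets the base color from the passed color, then restarts a timeline whose curves drive the material's opacity, ring and line parameters each update.
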(event `self.ReceiveBeginPlay`
  (bind _staticmeshcomponent (`self.StaticMeshComponent`))
  (bind _returnvalue (`PrimitiveComponent.CreateDynamicMaterialInstance` _staticmeshcomponent 0 (`PrimitiveComponent.GetMaterial` _staticmeshcomponent 0) "None"))
  (set `self.dynamicMaterialInstance` _returnvalue))

(event `PlayEffect`
  (params (color :type "LinearColor Structure"))
  (bind _dynamicmaterialinstance (`self.dynamicMaterialInstance`))
  (`/Engine/EditorBlueprintResources/StandardMacros.IsValid` (`self.dynamicMaterialInstance`)
    (:`Is Valid`
      (`MaterialInstanceDynamic.SetVectorParameterValue` (`self.dynamicMaterialInstance`) "baseColor" color)
      (bind (_direction _opacity _ringy _herolineamount _line_area_height _ringsize _lineareay _ringintensity) (`Timeline|effectOverTime` :!via `PlayFromStart`)
        (:`Update`
          (`|ExecutionSequence`
            (:`then_0`
              (`MaterialInstanceDynamic.SetScalarParameterValue` _dynamicmaterialinstance "masterOpacity" _opacity))
            (:`then_1`
              (`MaterialInstanceDynamic.SetScalarParameterValue` _dynamicmaterialinstance "RingBaseY" _ringy))
            (:`then_2`
              (`MaterialInstanceDynamic.SetScalarParameterValue` _dynamicmaterialinstance "heroLineAmount" _herolineamount))
            (:`then_3`
              (`MaterialInstanceDynamic.SetScalarParameterValue` _dynamicmaterialinstance "lineAreaSize" _line_area_height))
            (:`then_4`
              (`MaterialInstanceDynamic.SetScalarParameterValue` _dynamicmaterialinstance "RingWidth" _ringsize))
            (:`then_5`
              (`MaterialInstanceDynamic.SetScalarParameterValue` _dynamicmaterialinstance "LineAreaBaseY" _lineareay))
            (:`then_6`
              (`MaterialInstanceDynamic.SetScalarParameterValue` _dynamicmaterialinstance "ring_intensity_Mult" _ringintensity))))))))

(fn `UserConstructionScript`)