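; BP_Lightpillar is an interactable light pillar whose statue glows and then emits a light beam when activated.
; On BeginPlay it creates a dynamic material instance on the statue mesh.
; The first Interact sets an Active flag, blocking repeats, and plays a timeline driving the material's glow parameter.
; SpawnLightbeam runs when the timeline finishes, or immediately if the glow material is invalid.
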(event `self.ReceiveBeginPlay`
  (bind _statue (`self.statue`))
  ;[1 1 1] get material for glow
  (`parent.ReceiveBeginPlay`)
  (bind _returnvalue (`PrimitiveComponent.CreateDynamicMaterialInstance` _statue 0 (`PrimitiveComponent.GetMaterial` _statue 0) "None"))
  (set `self.glowMaterial` _returnvalue))

(event `/Game/Blueprints/Interface/BPI_Interact.Interact`
  (params (Actor :type "Actor Object Reference"))
  ;[1 1 1] allready activated?
  (if (not (`self.active`))
    (set `self.active` true)
    ;[1 1 1] let statue glow
    (`/Engine/EditorBlueprintResources/StandardMacros.IsValid` (`self.glowMaterial`)
      (:`Is Valid`
        (bind (_direction _newtrack_0) (`Timeline|glowTL`)
          (:`Update`
            (`MaterialInstanceDynamic.SetScalarParameterValue` (`self.glowMaterial`) "glow" _newtrack_0))
          (:`Finished`
            ;[1 1 1] spawn lighbeam
            (`self.SpawnLightbeam` :!label _label))))
      (:`Is Not Valid`
        (goto _label)))))

(fn `UserConstructionScript`
  (`parent.UserConstructionScript`))