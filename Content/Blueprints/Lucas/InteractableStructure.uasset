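; InteractableStructure is a one-shot discoverable world structure that registers with BP_DesignGameMode on BeginPlay.
; On first Interact it reports the find to the game mode, plays a sound at its location, sets its point light intensity and toggles the Ewew component's visibility.
; It also shows a HUD widget with text from the game mode, faded in and out by a timeline, then removed.
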(event `self.ReceiveBeginPlay`
  (bind _asbp_design_game_mode (cast `/Game/Blueprints/Lucas/BP_DesignGameMode` (`GameplayStatics.GetGameMode`)))
  (`/Game/Blueprints/Lucas/BP_DesignGameMode.RegisterInteractableStructure` _asbp_design_game_mode))

(event `/Game/Blueprints/Interface/BPI_Interact.Interact`
  (params (Actor :type "Actor Object Reference"))
  (if (not (`self.acticated`))
    (set `self.acticated` true)
    (`|ExecutionSequence`
      (:`then_0`
        (bind _asbp_design_game_mode (cast `/Game/Blueprints/Lucas/BP_DesignGameMode` (`GameplayStatics.GetGameMode`))
          (:`then`
            (`/Game/Blueprints/Lucas/BP_DesignGameMode.FindInteractableStructure` _asbp_design_game_mode))
          (:`CastFailed`
            (`GameplayStatics.PlaySound2D` null 1.0 1.0 0.0 null null))))
      (:`then_1`
        (`GameplayStatics.PlaySoundAtLocation` "/Game/Blueprints/Lucas/InteractableStructureSound.InteractableStructureSound" (`self.K2_GetActorLocation`) (struct) 1.0 1.0 0.0 null null null)
        (`LightComponent.SetIntensity` (`self.PointLight`) 5000.0)
        (`SceneComponent.ToggleVisibility` (`self.ewew`) false)
        (bind _displaytext (`/Game/Blueprints/Lucas/BP_DesignGameMode.GetInteractableStructureOnFindText` _asbp_design_game_mode))
        (bind _returnvalue (`|CreateWidget` "/Game/UI/WBP_InteractableStructure_HUD.WBP_InteractableStructure_HUD_C" null _displaytext))
        (`UserWidget.AddToViewport` _returnvalue 0)
        (bind (_direction _opacity) (`Timeline|TL_FadeInAndOut` :`NewTime` 1.0)
          (:`Update`
            (`Widget.SetRenderOpacity` _returnvalue _opacity))
          (:`Finished`
            (`Widget.RemoveFromParent` _returnvalue)))))))

(fn `UserConstructionScript`)