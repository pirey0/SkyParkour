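; BP_MovingStone moves its owning actor vertically, alternating between two phases like a floating or bobbing stone.
; BeginPlay runs an endless Delay loop that flips the Turn flag every FlightLenght seconds.
; Tick offsets the owner's Z location by the current speed without sweeping, then selects MoveSpeedUp or MoveSpeedDown from Turn.
; The offset is not scaled by delta time, so travel depends on frame rate.
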(event `self.ReceiveTick`
  (params (DeltaSeconds :type "Float (single-precision)"))
  (bind _returnvalue (`self.GetOwner`))
  (`Actor.K2_SetActorLocation` _returnvalue (+ (`Actor.K2_GetActorLocation` _returnvalue) (`KismetMathLibrary.MakeVector` 0.0 0.0 (`self.Internal Movement Speed`))) false false)
  (if (`self.Turn`)
    (set `self.Internal Movement Speed` (`self.Move Speed Up`))
    (else
      (set `self.Internal Movement Speed` (`self.Move Speed Down`)))))

(event `self.ReceiveBeginPlay`
  (bind _flight_lenght (`self.Flight Lenght`))
  (set `self.Internal Movement Speed` (`self.Move Speed Up`))
  (set `self.Turn` true :!label _label)
  (`KismetSystemLibrary.Delay` _flight_lenght)
  (set `self.Turn` false)
  (`KismetSystemLibrary.Delay` _flight_lenght)
  (goto _label))