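; BP_FunctionLibrary is a Blueprint function library with helpers for climb direction and component owner lookup.
; VectorToClimbDirection maps a vector to a climb direction enum using its dominant axis and the sign of Y or Z.
; Zero and X-dominant vectors share one enum value, so only the Y and Z axes yield signed directions.
; GetOwnerOrNull returns a component's owner after a validity check.
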(fn `GetOwnerOrNull`
  (params (Comp :type "ActorComponent Object Reference"))
  (returns (Actor :type "Actor Object Reference"))
  (`/Engine/EditorBlueprintResources/StandardMacros.IsValid` Comp
    (:`Is Valid`
      (return (`ActorComponent.GetOwner` Comp)))
    (:`Is Not Valid`
      (return null))))

(fn `VectorToClimbDirection`
  (params (Vector :type "Vector Structure"))
  (returns (Direction :type "/Game/Data/E_ClimbDirection Enum"))
  (locals (AbsX :type "Float (double-precision)") (AbsY :type "Float (double-precision)") (AbsZ :type "Float (double-precision)"))
  (`|ExecutionSequence`
    (:`then_0`
      (if (<= (`KismetMathLibrary.VSize` Vector) 0.0)
        (return "NewEnumerator4")))
    (:`then_1`
      (set `local.AbsX` (`KismetMathLibrary.Abs` (.x Vector))))
    (:`then_2`
      (set `local.AbsY` (`KismetMathLibrary.Abs` (.y Vector))))
    (:`then_3`
      (set `local.AbsZ` (`KismetMathLibrary.Abs` (.z Vector))))
    (:`then_4`
      (if (and (> (`local.AbsX`) (`local.AbsY`)) (> (`local.AbsX`) (`local.AbsZ`)))
        (return "NewEnumerator4")
        (elif (> (`local.AbsY`) (`local.AbsZ`))
          (if (< (.y Vector) 0.0)
            (return "NewEnumerator1")
            (else
              (return "NewEnumerator3")))
          (elif (> (.z Vector) 0.0)
            (return "NewEnumerator0")
            (else
              (return "NewEnumerator2"))))))))