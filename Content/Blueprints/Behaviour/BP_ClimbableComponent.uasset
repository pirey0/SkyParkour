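; Climbable component that links its owner to neighbouring climbables in up, right, down and left directions, forming a graph for climbing movement.
; On BeginPlay a sphere trace gathers nearby BPI_Climbable actors, and the best dot product in owner-local space picks each direction's reference.
; Getters return the neighbour in a direction and a climber transform in front of the owner, facing it.
; Links are drawn as coloured debug lines.
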(event `self.ReceiveBeginPlay`
  (`self.Calculate Reference Objects`)
  (`self.DebugDraw Connections` 1000000.0))

(fn `Calculate Reference Objects`
  (locals (NearbyClimbables :type "Array of Actor Object Reference"))
  (bind _nearbyclimbables (`local.NearbyClimbables`))
  (bind _returnvalue (`Actor.K2_GetActorLocation` (`self.GetOwner`)))
  (`|ExecutionSequence`
    (:`then_0`
      (`KismetSystemLibrary.PrintString` (`KismetStringLibrary.Concat_StrStr` (`KismetSystemLibrary.GetDisplayName` (`self.GetOwner`)) ": calculating Reference Objects")))
    (:`then_1`
      ;[1 1 1] Find and Store nearby Climbables
      (bind (_outhits _returnvalue_2) (`KismetSystemLibrary.SphereTraceMulti` :`Start` _returnvalue :`End` _returnvalue :`Radius` (`self.CheckTraceDistance`) :`TraceChannel` "TraceTypeQuery3" :`DrawDebugType` "ForDuration"))
      (if _returnvalue_2
        (for _array_element _outhits
          (bind (_bblockinghit _binitialoverlap _time _distance _location _impactpoint _normal _impactnormal _physmat _hitactor) (`GameplayStatics.BreakHitResult` _array_element))
          (if (`KismetSystemLibrary.DoesImplementInterface` _hitactor "/Game/Blueprints/Behaviour/BPI_Climbable.BPI_Climbable_C")
            (`KismetArrayLibrary.Array_Add` (`local.NearbyClimbables`) _hitactor)))))
    (:`then_2`
      ;[1 1 1] Assign References
      (`|ExecutionSequence`
        (:`then_0`
          (bind _bestactor (`self.GetBestForDirection` "NewEnumerator0" _nearbyclimbables))
          (bind _climbablecomp (message `/Game/Blueprints/Behaviour/BPI_Climbable.GetClimbableComponent` _bestactor))
          (set `self.UpReference` _climbablecomp))
        (:`then_1`
          (bind _bestactor_2 (`self.GetBestForDirection` "NewEnumerator1" _nearbyclimbables))
          (bind _climbablecomp_2 (message `/Game/Blueprints/Behaviour/BPI_Climbable.GetClimbableComponent` _bestactor_2))
          (set `self.RightReference` _climbablecomp_2))
        (:`then_2`
          (bind _bestactor_3 (`self.GetBestForDirection` "NewEnumerator2" _nearbyclimbables))
          (bind _climbablecomp_3 (message `/Game/Blueprints/Behaviour/BPI_Climbable.GetClimbableComponent` _bestactor_3))
          (set `self.DownReference` _climbablecomp_3))
        (:`then_3`
          (bind _bestactor_4 (`self.GetBestForDirection` "NewEnumerator3" _nearbyclimbables))
          (bind _climbablecomp_4 (message `/Game/Blueprints/Behaviour/BPI_Climbable.GetClimbableComponent` _bestactor_4))
          (set `self.LeftReference` _climbablecomp_4))))))

(fn `DebugDraw Connections`
  (params (Duration :type "Float (double-precision)"))
  (bind _returnvalue (`Actor.K2_GetActorLocation` (`self.GetOwner`)))
  (`|ExecutionSequence`
    (:`then_0`
      (bind _upreference (`self.UpReference`)
        (:`then`
          (`KismetSystemLibrary.DrawDebugLine` _returnvalue (`Actor.K2_GetActorLocation` (`self.GetOwner` _upreference)) (struct :`G` 0.054357 :`B` 1.0 :`A` 1.0) Duration 8.0))
        (:`else`)))
    (:`then_1`
      (bind _rightreference (`self.RightReference`)
        (:`then`
          (`KismetSystemLibrary.DrawDebugLine` _returnvalue (`Actor.K2_GetActorLocation` (`self.GetOwner` _rightreference)) (struct :`R` 1.0 :`G` 0.018187 :`A` 1.0) Duration 6.0))
        (:`else`)))
    (:`then_2`
      (bind _downreference (`self.DownReference`)
        (:`then`
          (`KismetSystemLibrary.DrawDebugLine` _returnvalue (`Actor.K2_GetActorLocation` (`self.GetOwner` _downreference)) (struct :`G` 0.770008 :`B` 1.0 :`A` 1.0) Duration 4.0))
        (:`else`)))
    (:`then_3`
      (bind _leftreference (`self.LeftReference`)
        (:`then`
          (`KismetSystemLibrary.DrawDebugLine` _returnvalue (`Actor.K2_GetActorLocation` (`self.GetOwner` _leftreference)) (struct :`R` 1.0 :`G` 0.372553 :`A` 1.0) Duration 2.0))
        (:`else`)))))

(fn `GetBestForDirection`
  (params (Direction :type "/Game/Data/E_ClimbDirection Enum" :default "NewEnumerator4") (Actors :type "Array of Actor Object Reference"))
  (returns (BestActor :type "Actor Object Reference"))
  (locals (TempBest :type "Actor Object Reference") (BestVal :type "Float (double-precision)"))
  (bind _returnvalue (`self.GetOwner`))
  (bind _vector (`/Game/Blueprints/Behaviour/BP_FunctionLibrary.DirectionToUnitVector` Direction))
  (for _array_element Actors
    (bind _returnvalue_2 (`KismetMathLibrary.Dot_VectorVector` _vector (`KismetMathLibrary.GreaterGreater_VectorRotator` (`KismetMathLibrary.GetDirectionUnitVector` (`Actor.K2_GetActorLocation` _returnvalue) (`Actor.K2_GetActorLocation` _array_element)) (`KismetMathLibrary.NegateRotator` (`Actor.K2_GetActorRotation` _returnvalue)))))
    (if (> _returnvalue_2 (`local.BestVal`))
      (set `local.BestVal` _returnvalue_2)
      (set `local.TempBest` _array_element)))
  (return (`local.TempBest`)))

(fn `GetClimbableInDirection`
  (params (Direction :type "/Game/Data/E_ClimbDirection Enum" :default "NewEnumerator4"))
  (returns (OutActor :type "Actor Object Reference"))
  (switch `/Game/Data/E_ClimbDirection` Direction
    (:`NewEnumerator4`
      (return null))
    (:`NewEnumerator0`
      (bind _actor (`/Game/Blueprints/Behaviour/BP_FunctionLibrary.GetOwnerOrNull` (`self.UpReference`)))
      (return _actor))
    (:`NewEnumerator1`
      (bind _actor_2 (`/Game/Blueprints/Behaviour/BP_FunctionLibrary.GetOwnerOrNull` (`self.RightReference`)))
      (return _actor_2))
    (:`NewEnumerator2`
      (bind _actor_3 (`/Game/Blueprints/Behaviour/BP_FunctionLibrary.GetOwnerOrNull` (`self.DownReference`)))
      (return _actor_3))
    (:`NewEnumerator3`
      (bind _actor_4 (`/Game/Blueprints/Behaviour/BP_FunctionLibrary.GetOwnerOrNull` (`self.LeftReference`)))
      (return _actor_4))))

(fn `GetClimberPosition`
  (returns (Position :type "Vector Structure"))
  (bind _returnvalue (`self.GetOwner`))
  (return (+ (`Actor.K2_GetActorLocation` _returnvalue) (* (`Actor.GetActorForwardVector` _returnvalue) 50.0))))

(fn `GetClimberRotation`
  (returns (Rotation :type "Rotator Structure"))
  (return (`KismetMathLibrary.Conv_VectorToRotator` (* (`KismetMathLibrary.Conv_RotatorToVector` (`Actor.K2_GetActorRotation` (`self.GetOwner`))) -1.0))))

(fn `GetOffsetDirection`
  (params (InActor :type "Actor Object Reference"))
  (returns (Direction :type "/Game/Data/E_ClimbDirection Enum"))
  (bind _returnvalue (`self.GetOwner`))
  (bind _direction (`/Game/Blueprints/Behaviour/BP_FunctionLibrary.VectorToClimbDirection` (`KismetMathLibrary.GreaterGreater_VectorRotator` (`KismetMathLibrary.GetDirectionUnitVector` (`Actor.K2_GetActorLocation` _returnvalue) (`Actor.K2_GetActorLocation` InActor)) (`KismetMathLibrary.NegateRotator` (`Actor.K2_GetActorRotation` _returnvalue)))))
  (return _direction))