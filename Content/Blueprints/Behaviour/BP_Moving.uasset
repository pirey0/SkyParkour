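; BP_Moving is a behaviour component that makes its owning actor bob up and down around the location it had at BeginPlay.
; BeginPlay stores that start position and picks a random phase offset, so instances move out of sync.
; Each Tick sets the owner's location, without sweep, to the start plus a Z-only sine of game time, scaled by speed and amplitude variables.
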(event `self.ReceiveTick`
  (params (DeltaSeconds :type "Float (single-precision)"))
  (`Actor.K2_SetActorLocation` (`self.GetOwner`) (+ (`self.StartPosition`) (`KismetMathLibrary.MakeVector` 0.0 0.0 (* (`KismetMathLibrary.DegSin` (+ (* (`GameplayStatics.GetTimeSeconds`) (`self.DegreesPerSec`)) (`self.Offset`))) (`self.MoveAmound`)))) false false))

(event `self.ReceiveBeginPlay`
  (set `self.StartPosition` (`Actor.K2_GetActorLocation` (`self.GetOwner`)))
  (set `self.Offset` (* (`KismetMathLibrary.RandomFloat`) 360.0)))