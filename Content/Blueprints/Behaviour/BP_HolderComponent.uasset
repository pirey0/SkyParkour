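; Holder component that lets its owner pick up a component, preview where it will go, and drop it there.
; Pickup snaps the item to a joint on the target mesh and disables its physics and collision.
; Update adjusts yaw and box-traces along the view rotation, caching the hit or max-range location and drawing it as a debug box.
; Drop detaches the item, restores physics, teleports it to that transform and plays a sound.
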(event `self.ReceiveTick`
  (params (DeltaSeconds :type "Float (single-precision)")))

(fn `CanPlace`
  (params (Start :type "Vector Structure") (Direction :type "Vector Structure") (maxDist :type "Float (double-precision)"))
  (returns (CanPlace :type Boolean) (Location :type "Vector Structure"))
  (`/Engine/EditorBlueprintResources/StandardMacros.IsValid` (`self.CurrentHeld`)
    (:`Is Valid`
      (bind (_outhit _returnvalue) (`KismetSystemLibrary.BoxTraceSingle` Start (+ (* Direction maxDist) Start) (`BoxComponent.GetScaledBoxExtent` (`self.CurrentHeld`)) (struct) "TraceTypeQuery1" false (`|MakeArray` (`self.GetOwner` (`self.TargetMesh`)) (`self.GetOwner` (`self.CurrentHeld`)))))
      (bind (_bblockinghit _binitialoverlap _time _distance _location _impactpoint _normal _impactnormal _physmat _hitactor) (`GameplayStatics.BreakHitResult` _outhit))
      (`KismetSystemLibrary.PrintString` (`KismetSystemLibrary.GetDisplayName` _hitactor) true true (struct :`G` 0.66 :`B` 1.0 :`A` 1.0) 0.05)
      (return _returnvalue _location))
    (:`Is Not Valid`
      (return false (0.0 0.0 0.0)))))

(fn `Drop`
  (bind _currentheld (`self.CurrentHeld`))
  (bind _currentheld_2 (`self.CurrentHeld`))
  (`/Engine/EditorBlueprintResources/StandardMacros.IsValid` _currentheld_2
    (:`Is Valid`
      (`SceneComponent.K2_DetachFromComponent` _currentheld_2 "KeepWorld" "KeepWorld" "KeepWorld" true)
      (`PrimitiveComponent.SetSimulatePhysics` _currentheld true)
      (`PrimitiveComponent.SetCollisionEnabled` _currentheld "QueryAndPhysics")
      (`SceneComponent.K2_SetWorldLocation` _currentheld (`self.LastLocation`) false true)
      (`SceneComponent.K2_SetWorldRotation` _currentheld (`self.LastRotation`) false true)
      (set `self.CurrentHeld` null)
      (`GameplayStatics.PlaySoundAtLocation` "/Game/Blueprints/DesignPrototype/plonk.plonk" (`self.LastLocation`) (struct) 3.0 1.0 0.0 null null null))))

(fn `IsHolding`
  (returns (isHolding :type Boolean) (Held :type "PrimitiveComponent Object Reference"))
  (bind _currentheld (`self.CurrentHeld`))
  (return (`KismetSystemLibrary.IsValid` _currentheld) _currentheld))

(fn `Pickup`
  (params (Comp :type "BoxComponent Object Reference"))
  (set `self.CurrentYaw` 90.0)
  (bind _output_get (set `self.CurrentHeld` Comp))
  (`SceneComponent.K2_AttachToComponent` _output_get (`self.TargetMesh`) (`KismetStringLibrary.Conv_StringToName` (`self.JointName`)) "SnapToTarget" "SnapToTarget" "KeepRelative" true)
  (`PrimitiveComponent.SetSimulatePhysics` (`local.Comp`) false)
  (`PrimitiveComponent.SetCollisionEnabled` (`local.Comp`) "NoCollision"))

(fn `Update`
  (params (Rotation :type "Rotator Structure") (CheckPosition :type "Vector Structure") (ExtraRotation :type "Float (double-precision)"))
  (bind _returnvalue (`KismetMathLibrary.GetForwardVector` Rotation))
  (bind _maxdistance (`self.MaxDistance`))
  (bind _returnvalue_2 (`BoxComponent.GetScaledBoxExtent` (`self.CurrentHeld`)))
  (bind _output_get (set `self.CurrentYaw` (+ (`self.CurrentYaw`) (* ExtraRotation (`self.RotationSpeedMultipyer`)))))
  (set `self.LastRotation` (`KismetMathLibrary.MakeRotator` 0.0 0.0 (+ (.yaw Rotation) _output_get)))
  (`/Engine/EditorBlueprintResources/StandardMacros.IsValid` (`self.CurrentHeld`)
    (:`Is Valid`
      (bind (_canplace _location) (`self.CanPlace` CheckPosition _returnvalue _maxdistance))
      (if _canplace
        (bind _output_get_2 (set `self.LastLocation` _location))
        (`KismetSystemLibrary.DrawDebugBox` _output_get_2 _returnvalue_2 (struct :`G` 1.0 :`B` 0.341191 :`A` 1.0) (`self.LastRotation`))
        (else
          (bind _output_get_3 (set `self.LastLocation` (+ (* _returnvalue _maxdistance) CheckPosition)))
          (`KismetSystemLibrary.DrawDebugBox` _output_get_3 _returnvalue_2 (struct :`G` 1.0 :`B` 0.341191 :`A` 1.0) (`self.LastRotation`)))))))