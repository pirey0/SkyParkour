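; BP_RandomAmbientSpawn is an ambient sound actor that plays a goose sound at random intervals.
; Tick accumulates elapsed time and, once it passes the current wait, plays the sound as non-positional 2D audio at boosted volume.
; It then resets the timer and picks a new random wait of seconds to minutes, with only a brief initial wait after BeginPlay.
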(event `self.ReceiveBeginPlay`
  (set `self.currentWaitTime` 1.0))

(event `self.ReceiveTick`
  (params (DeltaSeconds :type "Float (single-precision)"))
  (bind _output_get (set `self.passedTime` (+ DeltaSeconds (`self.passedTime`))))
  (if (> _output_get (`self.currentWaitTime`))
    (`GameplayStatics.SpawnSound2D` "/Game/SFX/Environment/S_Goose1.S_Goose1" 10.0 1.0 0.0 null)
    (set `self.currentWaitTime` (`KismetMathLibrary.RandomFloatInRange` 10.0 180.0))
    (set `self.passedTime` 0.0)))

(fn `UserConstructionScript`)