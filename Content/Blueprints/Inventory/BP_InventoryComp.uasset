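; Inventory component that gives its owner a fixed number of item slots, with queries, removal and bulk transfers to or from the player's inventory.
; Adds fill partial stacks of the same item name first, recursing on overflow, then take an empty slot, marked by a zero-count group.
; Adds and removals fire an InventoryChanged notification, and the component creates inventory window widgets bound to itself.
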(event `self.ReceiveBeginPlay`
  (`self.Setup`))

(fn `AddToInventory`
  (params (Element :type "/Game/Blueprints/Inventory/S_InventoryGroup Structure") (Log :type Boolean))
  (returns (WasAdded :type Boolean))
  (bind _element (`local.Element`))
  (if Log
    (`KismetSystemLibrary.PrintString` (`KismetStringLibrary.Concat_StrStr` (`KismetSystemLibrary.GetDisplayName` (`self.GetOwner`)) " trying to add " (`KismetStringLibrary.Conv_IntToString` Element_Count_6_994EF10D417449C7AE0816A2DAA774D6) " " (`KismetStringLibrary.Conv_NameToString` (break `/Game/Blueprints/Inventory/S_InventoryObject` (break `/Game/Blueprints/Inventory/S_InventoryGroup` Element)))) true true (struct :`G` 1.0 :`B` 0.570512 :`A` 1.0)))
  (if (`.IsStackable_12_E124494A450BF1C631100394484E1640` (break `/Game/Blueprints/Inventory/S_InventoryObject` (break `/Game/Blueprints/Inventory/S_InventoryGroup` Element)))
    (bind _stackindex (`self.HasPartialStack` _element)
      (:`True`
        (bind _success (`self.AddToStack` _element _stackindex))
        (`self.InventoryChanged`)
        (return _success))
      (:`False`
        _)))
  (bind _success_2 (`self.TryMakeNewStack` (`local.Element`)))
  (`self.InventoryChanged`)
  (return _success_2))

(fn `AddToStack`
  (params (Group :type "/Game/Blueprints/Inventory/S_InventoryGroup Structure") (StackIndex :type Integer))
  (returns (Success :type Boolean))
  (locals (CurrentCount :type Integer))
  (bind _group_inventoryobject (break `/Game/Blueprints/Inventory/S_InventoryGroup` (`local.Group`)))
  (bind (_group_inventoryobject_2 _group_count) (break `/Game/Blueprints/Inventory/S_InventoryGroup` (`local.Group`)))
  (bind _group_inventoryobject_3 (break `/Game/Blueprints/Inventory/S_InventoryGroup` (`local.Group`)))
  (bind (_name _description _thumbnail _isstackable _maxstacksize) (break `/Game/Blueprints/Inventory/S_InventoryObject` _group_inventoryobject_2))
  (bind _output (`|GetArrayItem` (`self.Inventory`) StackIndex))
  (bind _output_get (set `local.CurrentCount` (`.Count_6_994EF10D417449C7AE0816A2DAA774D6` (break `/Game/Blueprints/Inventory/S_InventoryGroup` _output))))
  (bind _returnvalue (+ _output_get (`.Count_6_994EF10D417449C7AE0816A2DAA774D6` (break `/Game/Blueprints/Inventory/S_InventoryGroup` Group))))
  (if (> _returnvalue (`.MaxStackSize_15_D9E3DD54451EE4E447B16E8DD9DF72C1` (break `/Game/Blueprints/Inventory/S_InventoryObject` (break `/Game/Blueprints/Inventory/S_InventoryGroup` _output))))
    (`KismetArrayLibrary.Array_Set` (`self.Inventory`) (`local.StackIndex`) (make `/Game/Blueprints/Inventory/S_InventoryGroup` _group_inventoryobject_2 _maxstacksize))
    ;[1 1 1] Recursively calls Add
    (bind _wasadded (`self.AddToInventory` (make `/Game/Blueprints/Inventory/S_InventoryGroup` _group_inventoryobject_3 (- _group_count (- _maxstacksize (`local.CurrentCount`))))))
    (return _wasadded)
    (else
      (`KismetArrayLibrary.Array_Set` (`self.Inventory`) (`local.StackIndex`) (make `/Game/Blueprints/Inventory/S_InventoryGroup` _group_inventoryobject _returnvalue))
      (return true))))

(fn `Contains`
  (params (Object :type "/Game/Blueprints/Inventory/S_InventoryObject Structure"))
  (returns (IsContained :type Boolean))
  (for _array_element (`self.Inventory`)
    (if (== (break `/Game/Blueprints/Inventory/S_InventoryObject` (break `/Game/Blueprints/Inventory/S_InventoryGroup` _array_element)) Object_Name_3_338EC17E460C2EBDBF6FE99A78DFD90E)
      (return true)))
  (return false))

(fn `Contains Atleast`
  (params (Group :type "/Game/Blueprints/Inventory/S_InventoryGroup Structure"))
  (returns (DoesContainAtleast :type Boolean))
  (locals (Remaining :type Integer))
  (set `local.Remaining` Group_Count_6_994EF10D417449C7AE0816A2DAA774D6)
  (for _array_element (`self.Inventory`)
    (if (== (break `/Game/Blueprints/Inventory/S_InventoryObject` (break `/Game/Blueprints/Inventory/S_InventoryGroup` _array_element)) (break `/Game/Blueprints/Inventory/S_InventoryObject` (break `/Game/Blueprints/Inventory/S_InventoryGroup` Group)))
      (bind _output_get (set `local.Remaining` (- (`local.Remaining`) (`.Count_6_994EF10D417449C7AE0816A2DAA774D6` (break `/Game/Blueprints/Inventory/S_InventoryGroup` _array_element)))))
      (if (<= _output_get 0)
        (return true))))
  (return false))

(fn `CreateInventoryWidget`
  (returns (NewParam :type "/Game/UI/Inventory/WBP_InventoryWindow Object Reference"))
  (bind _returnvalue (`|CreateWidget` "/Game/UI/Inventory/WBP_InventoryWindow.WBP_InventoryWindow_C" null self (`self.IsPlayer`)))
  (return _returnvalue))

(fn `RemoveStack`
  (params (Index :type Integer))
  (returns (RemovedGroup :type "/Game/Blueprints/Inventory/S_InventoryGroup Structure"))
  (locals (Copy :type "/Game/Blueprints/Inventory/S_InventoryGroup Structure"))
  (set `local.Copy` (`|GetArrayItem` (`self.Inventory`) Index))
  (`KismetArrayLibrary.Array_Set` (`self.Inventory`) Index (make `/Game/Blueprints/Inventory/S_InventoryGroup` (struct :`Name` "Default" :`IsStackable` true :`MaxStackSize` 64)))
  (`self.InventoryChanged`)
  (return (`local.Copy`)))

(fn `Setup`
  (`KismetArrayLibrary.Array_Resize` (`self.Inventory`) (`self.SlotCount`)))

(fn `TryMakeNewStack`
  (params (Element :type "/Game/Blueprints/Inventory/S_InventoryGroup Structure"))
  (returns (Success :type Boolean))
  (bind _inventory (`self.Inventory`))
  (bind _returnvalue (`KismetArrayLibrary.Array_Find` _inventory (make `/Game/Blueprints/Inventory/S_InventoryGroup` (struct :`Name` "Default" :`IsStackable` true :`MaxStackSize` 64))))
  (if (!= _returnvalue -1)
    (`KismetArrayLibrary.Array_Set` _inventory _returnvalue Element)
    (return true)
    (else
      (return false))))

(fn `TryRemove`
  (params (Group :type "/Game/Blueprints/Inventory/S_InventoryGroup Structure"))
  (returns (Removed :type Boolean))
  (locals (Remaining :type Integer))
  (bind _group_inventoryobject (break `/Game/Blueprints/Inventory/S_InventoryGroup` (`local.Group`)))
  (set `local.Remaining` Group_Count_6_994EF10D417449C7AE0816A2DAA774D6)
  (for (_array_element _array_index) (`self.Inventory`)
    (if (== (break `/Game/Blueprints/Inventory/S_InventoryObject` (break `/Game/Blueprints/Inventory/S_InventoryGroup` _array_element)) "None")
      (bind _output_get (set `local.Remaining` (- (`local.Remaining`) (`.Count_6_994EF10D417449C7AE0816A2DAA774D6` (break `/Game/Blueprints/Inventory/S_InventoryGroup` _array_element)))))
      (`|ExecutionSequence`
        (:`then_0`
          (if (>= _output_get 0)
            (`KismetArrayLibrary.Array_Set` (`self.Inventory`) _array_index (make `/Game/Blueprints/Inventory/S_InventoryGroup` (struct :`Name` "Default" :`IsStackable` true :`MaxStackSize` 64)))
            (else
              (`KismetArrayLibrary.Array_Set` (`self.Inventory`) _array_index (make `/Game/Blueprints/Inventory/S_InventoryGroup` _group_inventoryobject (* (`local.Remaining`) -1))))))
        (:`then_1`
          (if (<= _output_get 0)
            (`self.InventoryChanged`)
            (return true))))))
  (return false))

(fn `TryTakeAllFromPlayer`
  (if (not (`self.IsPlayer`))
    (bind _playerinventory (`/Game/Blueprints/Behaviour/BP_FunctionLibrary.GetPlayerInventory` (`self.GetOwner`)))
    (`/Engine/EditorBlueprintResources/StandardMacros.IsValid` _playerinventory
      (:`Is Valid`
        (`self.TryTransferAll` _playerinventory self)))))

(fn `TryTransferAll`
  (params (TargetInventory :type "/Game/Blueprints/Inventory/BP_InventoryComp Object Reference"))
  (`/Engine/EditorBlueprintResources/StandardMacros.IsValid` TargetInventory
    (:`Is Valid`
      (for (_array_element _array_index) (`self.Inventory`)
        (if (> (`.Count_6_994EF10D417449C7AE0816A2DAA774D6` (break `/Game/Blueprints/Inventory/S_InventoryGroup` _array_element)) 0)
          (bind _wasadded (`self.AddToInventory` (`local.TargetInventory`) _array_element true))
          (if _wasadded
            (`self.RemoveStack` _array_index)))))))

(fn `TryTransferAllToPlayer`
  (if (not (`self.IsPlayer`))
    (bind _playerinventory (`/Game/Blueprints/Behaviour/BP_FunctionLibrary.GetPlayerInventory` (`self.GetOwner`)))
    (`/Engine/EditorBlueprintResources/StandardMacros.IsValid` _playerinventory
      (:`Is Valid`
        (`self.TryTransferAll` _playerinventory)))))